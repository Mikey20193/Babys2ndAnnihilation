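; Multiplayer game instance that handles sessions, map travel and shared state for players, settings, selected mode and UI options.
; Advanced Sessions nodes create, find and join sessions, including invites, with hosts opening the lobby as a listen server.
; StartGame server-travels to a map matched from the mode name, and EndGame returns to the lobby.
; It also spawns menu and timer audio plus the round actor, and broadcasts input, role and UI changes.
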(event `Set Selected Game Mode`
  (params (`Selected Game Mode` :type "GameModeBase Class Reference"))
  (if (`Actor.HasAuthority` (`GameplayStatics.GetPlayerController` 0))
    (bind _output_get (set `self.Selected Game Mode` `Selected Game Mode`))
    (bind _returnvalue_pathstring (break `TopLevelAssetPath` (`KismetSystemLibrary.GetClassTopLevelAssetPath` _output_get)))
    (`KismetSystemLibrary.PrintString` _returnvalue_pathstring)
    (else
      (`KismetSystemLibrary.RaiseScriptError` "You have no authority here Jacqui Weaver"))))

(event `ROS_Add Player to active Players`
  (params (PCs :type "PlayerController Object Reference"))
  (`KismetArrayLibrary.Array_Add` (`self.PCs`) PCs))

(event `ROS_Remove Player from Active Players`
  (params (PCs :type "PlayerController Object Reference"))
  (`KismetArrayLibrary.Array_RemoveItem` (`self.PCs`) PCs))

(event `End Game`
  (`KismetSystemLibrary.Delay` 2.0)
  (if (`KismetSystemLibrary.IsServer`)
    (`AdvancedSessionsLibrary.ServerTravel` "Lvl_Lobby")))

(event `Start Game`
  (params (`Game Mode Name` :type String))
  (if (`KismetSystemLibrary.IsServer`)
    (if (`KismetStringLibrary.Contains` `Game Mode Name` "FFA")
      (`KismetSystemLibrary.ExecuteConsoleCommand` (`KismetStringLibrary.Concat_StrStr` "ServerTravel " (`KismetStringLibrary.Concat_StrStr` "Lvl_FFA?=" `Game Mode Name`)) null)
      (elif (`KismetStringLibrary.Contains` `Game Mode Name` "Tower")
        (`KismetSystemLibrary.ExecuteConsoleCommand` (`KismetStringLibrary.Concat_StrStr` "ServerTravel " (`KismetStringLibrary.Concat_StrStr` "LV_TowerDefense?=" `Game Mode Name`)) null)
        (elif (`KismetStringLibrary.Contains` `Game Mode Name` "King")
          (`KismetSystemLibrary.ExecuteConsoleCommand` (`KismetStringLibrary.Concat_StrStr` "ServerTravel " (`KismetStringLibrary.Concat_StrStr` "Lvl_Dom?=" `Game Mode Name`)) null)
          (elif (`KismetStringLibrary.Contains` `Game Mode Name` "Team")
            (`KismetSystemLibrary.ExecuteConsoleCommand` (`KismetStringLibrary.Concat_StrStr` "ServerTravel " (`KismetStringLibrary.Concat_StrStr` "Lvl_TDM?=" `Game Mode Name`)) null)))))))

(event `Update text Scale`
  (params (TextScaleFactor :type "Float (double-precision)"))
  (bind _output_get (set `self.TextScaleFactor` TextScaleFactor))
  (`self.OnTextScaleChanged` _output_get))

(event `Update Backplate Opacity`
  (params (`Backplate opacity` :type "Float (double-precision)"))
  (set `self.Global_Backplate_Opacity` `Backplate opacity`)
  (`self.OnBackplateOpacityChanged`))

(event `ReceiveInit_1`
  (bind _returnvalue (`GameplayStatics.SpawnSound2D` "/Game/Audio/Metasounds/Sources/MS_SFX_UI_MainMenu.MS_SFX_UI_MainMenu" 1.0 1.0 0.0 null true :!label _label))
  (set `self.MS_UI_MainMenu` _returnvalue)
  (bind _returnvalue_2 (`GameplayStatics.SpawnSound2D` null 1.0 1.0 0.0 null true))
  (set `self.MS_UI_PauseMenu` _returnvalue_2)
  (if (`self.bDebugging?`)
    (`KismetSystemLibrary.ExecuteConsoleCommand` "EnableAllScreenMessages" null)
    (else
      (`KismetSystemLibrary.ExecuteConsoleCommand` "DisableAllScreenMessages" null))))

(event `InitAudio`
  (goto _label))

(event `Create Session`
  (bind _returnvalue (`GameplayStatics.GetPlayerController` 0))
  (`DestroySessionCallbackProxy.DestroySession` _returnvalue
    (:`OnSuccess`
      _)
    (:`OnFailure`
      (`KismetSystemLibrary.PrintString` "no server to destroy")))
  (if (`Controller.IsLocalPlayerController` _returnvalue)
    (`CreateSessionCallbackProxyAdvanced.CreateAdvancedSession` :`PlayerController` _returnvalue :`PublicConnections` 10 :`bAllowJoinViaPresenceFriendsOnly` true :`bUseLobbiesVoiceChatIfAvailable` true
      (:`OnSuccess`
        (`KismetSystemLibrary.PrintString` "Server Created and Listening")
        (`GameplayStatics.OpenLevelBySoftObjectPtr` "/Game/Levels/Lvl_Lobby.Lvl_Lobby" true "?listen")))))

(event `/Game/Blueprints/GameArchitecture/BPI/BPI_TowerDefenseInst.SetSettings`
  (params (NewSettings :type "/Game/Blueprints/GameArchitecture/Settings/BP_GameSettings Class Reference"))
  (set `self.GameSettings` NewSettings))

(event `Controller Input Detected`
  (params (IsUsingPad :type Boolean) (IsUsingKBM :type Boolean))
  (set `self.IsUsingKBM` IsUsingKBM)
  (set `self.IsUsingGamepad` IsUsingPad)
  (`self.OnInputModeChanged` (`self.IsUsingKBM`) (`self.IsUsingGamepad`)))

(event `CustomEvent_1`
  (params (`Number Of Players` :type Integer))
  (set `self.NumberOfLocalPlayer` `Number Of Players`))

(event `OnSessionInviteAccepted_1`
  (params (LocalPlayerNum :type Integer) (PersonInvited :type "BPUniqueNetId Structure") (SessionToJoin :type "BlueprintSessionResult Structure (by ref)"))
  (`JoinSessionCallbackProxy.JoinSession` (`GameplayStatics.GetPlayerController` 0) SessionToJoin))

(event `Join Session`
  (bind _returnvalue (`GameplayStatics.GetPlayerController` 0))
  (bind _results (`FindSessionsCallbackProxyAdvanced.FindSessionsAdvanced` :`PlayerController` _returnvalue :`MaxResults` 10 :`ServerTypeToSearch` "AllServers" :`MinSlotsAvailable` 1)
    (:`OnSuccess`
      (`JoinSessionCallbackProxy.JoinSession` _returnvalue (`|GetArrayItem` _results)
        (:`then`
          (`KismetSystemLibrary.Delay` 4.0)
          (bind _output_get (set `self.Is Client? ` true))
          (`self.OnServerRoleChanged?` _output_get))))))

(event `self.OnSessionInviteAccepted`
  (params (LocalPlayerNum :type Integer) (PersonInvited :type "BPUniqueNetId Structure") (SessionToJoin :type "BlueprintSessionResult Structure (by ref)"))
  (bind _returnvalue (`GameplayStatics.GetPlayerController` 0))
  (`DestroySessionCallbackProxy.DestroySession` _returnvalue
    (:`OnSuccess`
      _)
    (:`OnFailure`
      _))
  (`JoinSessionCallbackProxy.JoinSession` _returnvalue SessionToJoin
    (:`then`
      (`KismetSystemLibrary.Delay` 4.0)
      (bind _output_get (set `self.Is Client? ` true))
      (`self.OnServerRoleChanged?` _output_get))))

(event `ROS_Create Game Audio`
  (bind _returnvalue (`GameplayStatics.SpawnSound2D` "/Game/Audio/Metasounds/Sources/MS_SFX_UI_Timer.MS_SFX_UI_Timer" 1.0 1.0 0.0 null false false))
  (set `self.RoundTimer` _returnvalue))

(event `ROS_CreateRound`
  (`self.Current Round`
    (:`then`)
    (:`else`
      (bind _returnvalue (`|SpawnActorFromClass` "/Game/Blueprints/Actors/BP_Round.BP_Round_C" (`KismetMathLibrary.MakeTransform` (0.0 0.0 0.0)) "Undefined" "MultiplyWithRoot" null null))
      (set `self.Current Round` _returnvalue))))

(fn `GetActivePlayers`
  (returns (PCs :type "Array of PlayerController Object Reference"))
  (return (`self.PCs`)))

(fn `GetGameSettings`
  (returns (GameSettings :type "/Game/Blueprints/GameArchitecture/Settings/BP_GameSettings Class Reference"))
  (return (`self.GameSettings`)))

(fn `GetNumberOfLocalPlayers`
  (returns (`Number Of Local Players` :type Integer))
  (return 0))