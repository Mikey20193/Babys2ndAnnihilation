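; BP_Wind_Test is a test wind volume that pushes the first-person character while inside its box.
; Box overlaps add or remove characters from AffectedActors and toggle ShouldApplyWind, which any single exit clears.
; Tick applies WindDirection as a velocity-change impulse to each listed character's movement component.
; A random gust routine jitters horizontal wind and prints it, but its FluxuateWind trigger is never run.
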(event `self.Box.OnComponentEndOverlap`
  (params (OverlappedComponent :type "PrimitiveComponent Object Reference") (OtherActor :type "Actor Object Reference") (OtherComp :type "PrimitiveComponent Object Reference") (OtherBodyIndex :type Integer))
  (bind _asbp_first_person_character (cast `/Game/FirstPerson/Blueprints/BP_FirstPersonCharacter` OtherActor))
  (set `self.ShouldApplyWind?` false)
  (`KismetArrayLibrary.Array_RemoveItem` (`self.Affected Actors`) _asbp_first_person_character))

(event `self.Box.OnComponentBeginOverlap`
  (params (OverlappedComponent :type "PrimitiveComponent Object Reference") (OtherActor :type "Actor Object Reference") (OtherComp :type "PrimitiveComponent Object Reference") (OtherBodyIndex :type Integer) (bFromSweep :type Boolean) (SweepResult :type "HitResult Structure (by ref)"))
  (bind _asbp_first_person_character (cast `/Game/FirstPerson/Blueprints/BP_FirstPersonCharacter` OtherActor))
  (`KismetArrayLibrary.Array_Add` (`self.Affected Actors`) _asbp_first_person_character)
  (set `self.ShouldApplyWind?` true))

(event `self.ReceiveTick`
  (params (DeltaSeconds :type "Float (single-precision)"))
  (if (`self.ShouldApplyWind?`)
    (`self.Apply wind`)))

(event `Apply wind`
  (for _array_element (`self.Affected Actors`)
    (`CharacterMovementComponent.AddImpulse` (`Character.CharacterMovement` _array_element) (`self.Wind Direction`) true)))

(event `Randomize Wind Speed`
  (bind (_wind_direction_x _wind_direction_y _wind_direction_z) (`KismetMathLibrary.BreakVector` (`self.Wind Direction`)))
  (bind _output_get (set `self.Wind Direction` (`KismetMathLibrary.MakeVector` (+ _wind_direction_x (`KismetMathLibrary.RandomFloatInRange` -10.0 10.0)) (+ _wind_direction_y (`KismetMathLibrary.RandomFloatInRange` -10.0 10.0)) _wind_direction_z)))
  (`KismetSystemLibrary.PrintString` (`KismetStringLibrary.Concat_StrStr` "Wind Speed" (`KismetStringLibrary.Conv_VectorToString` _output_get))))

(event `Fluxuate Wind`
  (bind _output_get (set `self.Should Fluxuate` (> (`KismetMathLibrary.RandomIntegerInRange` 0 4) 3)))
  (if _output_get
    (`self.Randomize Wind Speed`)
    (set `self.Should Fluxuate` false)))

(fn `UserConstructionScript`)