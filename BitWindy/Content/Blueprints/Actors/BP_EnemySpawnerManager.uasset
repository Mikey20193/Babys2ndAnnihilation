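; Manager actor for tower defense enemy waves that groups level spawners into buckets by target tower and spawns from them when the spawn interval is reached.
; Each wave rotates across buckets, offset by wave number, using each bucket's least-used spawner.
; Wave size starts from GameMode difficulty settings and grows periodically to a cap.
; It reports enemy spawns and KOs as count changes, and toggles spawner charge sounds with rounds.
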(event `self.ReceiveBeginPlay`
  ; Comment
  (`self.SetUpSpawnerMap`)
  (`self.SetUpWaveLogic`)
  (bind _asbp_tower_defense_game_mode (cast `/Game/Blueprints/GameArchitecture/BP_TowerDefense_GameMode` (`GameplayStatics.GetGameMode`)))
  (bind _bp_roundmanager_basic_hud (`/Game/Blueprints/GameArchitecture/BP_TowerDefense_GameMode.BP_RoundManager_Basic_HUD` _asbp_tower_defense_game_mode))
  (add `/Game/Blueprints/GameArchitecture/Components/BP_RoundManager_Basic_HUD.RoundBegin` _bp_roundmanager_basic_hud (`|CreateDelegate` :!event `Round Begun`))
  (add `/Game/Blueprints/GameArchitecture/Components/BP_RoundManager_Basic_HUD.RoundOver` _bp_roundmanager_basic_hud (`|CreateDelegate` :!event `Round Over`)))

(event `OnEnemySpawnIntervalReached`
  ; Listen to Round
  (`self.HandleEnemySpawning`))

(event `OnEnemyKOed`
  ; Tell GameState to change enemy count
  (`self.EnemyCountDecreased`))

(fn `ChooseSpawnerInBucket`
  (params (Bucket :type "/Game/Blueprints/GameArchitecture/Components/BP_SpawnerBucket Object Reference"))
  (returns (ChosenSpawner :type "/Game/Blueprints/Actors/BP_EnemySpawner Object Reference"))
  (bind _spawner (`/Game/Blueprints/GameArchitecture/Components/BP_SpawnerBucket.GetLeastUsedSpawner` Bucket))
  (return _spawner))

(fn `HandleEnemySpawning`
  (bind _keys (`BlueprintMapLibrary.Map_Keys` (`self.SpawnersByTargetMap`)))
  (for _index (range 1 (+ (`self.Enemies Per Wave`) 1))
    (bind _chosenbucket (`self.PickNextBucket` _index _keys))
    (bind _chosenspawner (`self.ChooseSpawnerInBucket` _chosenbucket))
    (bind (_bsuccessful _spawnedenemyref) (`/Game/Blueprints/Actors/BP_EnemySpawner.Spawn Enemy ` _chosenspawner))
    (if _bsuccessful
      (message `/Game/Variant_Shooter/Blueprints/AI/BPI_InitTowerDefenseEnemy.BindEventToKODispatcher` _spawnedenemyref self)
      (`self.EnemyCountIncreased`)
      (else
        (`KismetSystemLibrary.RaiseScriptError` (`KismetStringLibrary.Concat_StrStr` "Enemy Spawn Failed -  " (`KismetStringLibrary.Conv_ObjectToString` _chosenspawner) " produced invalid result")))))
  (`self.IncrementWave`))

(fn `IncrementWave`
  (bind _result (`/Engine/EditorBlueprintResources/StandardMacros.IncrementInt` (`self.CurrentWave`))
    (:`  `
      (if (< (`self.Enemies Per Wave`) (`self.Cap`))
        (if (== 0 (mod _result (`self.Increment Interval`)))
          (`/Engine/EditorBlueprintResources/StandardMacros.IncrementInt` (`self.Enemies Per Wave`)))))))

(fn `PickNextBucket`
  (params (EnemiesSpawnedThisWave :type Integer) (BucketKeys :type "Array of /Game/Data/ETower Enum"))
  (returns (ChosenBucket :type "/Game/Blueprints/GameArchitecture/Components/BP_SpawnerBucket Object Reference"))
  (return (`BlueprintMapLibrary.Map_Find` (`self.SpawnersByTargetMap`) (`|GetArrayItem` BucketKeys (mod (+ EnemiesSpawnedThisWave (`self.CurrentWave`)) (`KismetArrayLibrary.Array_Length` BucketKeys))))))

(fn `Round Begun`
  (params (RoundNumber :type Integer) (TimeInRound :type "Float (double-precision)") (bBetweenRound :type Boolean))
  (if (not bBetweenRound)
    (bind (_keypin _valuepin) (`|MapForEach` (`self.SpawnersByTargetMap`))
      (:`then`
        (for _array_element (`/Game/Blueprints/GameArchitecture/Components/BP_SpawnerBucket.Spawners` _valuepin)
          (`/Game/Blueprints/Actors/BP_EnemySpawner.PlayChargeSound` _array_element))))))

(fn `Round Over`
  (params (RoundNumber :type Integer))
  (bind (_keypin _valuepin) (`|MapForEach` (`self.SpawnersByTargetMap`))
    (:`then`
      (for _array_element (`/Game/Blueprints/GameArchitecture/Components/BP_SpawnerBucket.Spawners` _valuepin)
        (`/Game/Blueprints/Actors/BP_EnemySpawner.Stop Charge Sound` _array_element)))))

(fn `SetUpSpawnerMap`
  (locals (SpawnerActor :type "/Game/Blueprints/Actors/BP_EnemySpawner Object Reference"))
  (bind _targettower (`/Game/Blueprints/Actors/BP_EnemySpawner.TargetTower` (`local.SpawnerActor`)))
  (bind (_value _returnvalue) (`BlueprintMapLibrary.Map_Find` (`self.SpawnersByTargetMap`) _targettower))
  (bind _outactors (`GameplayStatics.GetAllActorsOfClass` "/Game/Blueprints/Actors/BP_EnemySpawner.BP_EnemySpawner_C"))
  (for _array_element _outactors
    (set `local.SpawnerActor` _array_element)
    (if _returnvalue
      (`/Game/Blueprints/GameArchitecture/Components/BP_SpawnerBucket.AddSpawner` _value (`local.SpawnerActor`))
      (else
        (bind _returnvalue_2 (`|GenericCreateObject` "/Game/Blueprints/GameArchitecture/Components/BP_SpawnerBucket.BP_SpawnerBucket_C"))
        (bind _bucketref (`/Game/Blueprints/GameArchitecture/Components/BP_SpawnerBucket.AddSpawner` _returnvalue_2 (`local.SpawnerActor`)))
        (`BlueprintMapLibrary.Map_Add` (`self.SpawnersByTargetMap`) _targettower _bucketref))))
  (if (== (`BlueprintMapLibrary.Map_Length` (`self.SpawnersByTargetMap`)) 0)
    (`KismetSystemLibrary.RaiseScriptError` "No Enemy Spawners Found")))

(fn `SetUpWaveLogic`
  (bind _difficulty_settings (message `/Game/Blueprints/GameArchitecture/BPI/BPI_TowerDefenseGameMode.GetDifficultySettings` (`GameplayStatics.GetGameMode`)))
  (bind (_roundstotal _basetimelimit _timitlimitincrement _basespawnfrequency _spawnfrequencydecrement _baseenemiesperwave _wavesizeincrementinterval _wavesizecap) (break `/Game/Data/F_DifficultySettings` _difficulty_settings))
  (set `self.Enemies Per Wave` _baseenemiesperwave)
  (set `self.Increment Interval` _wavesizeincrementinterval)
  (set `self.Cap` _wavesizecap))

(fn `UserConstructionScript`)