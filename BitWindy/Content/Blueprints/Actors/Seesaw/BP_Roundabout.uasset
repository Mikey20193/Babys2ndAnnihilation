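; BP_Roundabout is a roundabout actor that spins while a BP_ShooterCharacter is on its trigger.
; Begin and end overlaps on the Wwe component set and clear the ShouldRotate flag.
; While the flag is set, Tick increases Cylinder1's relative yaw by DeltaSeconds plus a constant, so spin speed depends on frame rate.
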(event `self.ReceiveTick`
  (params (DeltaSeconds :type "Float (single-precision)"))
  (bind _cylinder1 (`self.Cylinder1`))
  (bind (_relativerotation_roll _relativerotation_pitch _relativerotation_yaw) (`KismetMathLibrary.BreakRotator` (`SceneComponent.RelativeRotation` _cylinder1)))
  (if (`self.Should rotate`)
    (`SceneComponent.K2_SetRelativeRotation` _cylinder1 (`KismetMathLibrary.MakeRotator` _relativerotation_roll _relativerotation_pitch (+ _relativerotation_yaw (+ DeltaSeconds 2.0))) false false)))

(event `self.wwe.OnComponentBeginOverlap`
  (params (OverlappedComponent :type "PrimitiveComponent Object Reference") (OtherActor :type "Actor Object Reference") (OtherComp :type "PrimitiveComponent Object Reference") (OtherBodyIndex :type Integer) (bFromSweep :type Boolean) (SweepResult :type "HitResult Structure (by ref)"))
  (cast `/Game/Variant_Shooter/Blueprints/BP_ShooterCharacter` OtherActor)
  (set `self.Should rotate` true))

(event `self.wwe.OnComponentEndOverlap`
  (params (OverlappedComponent :type "PrimitiveComponent Object Reference") (OtherActor :type "Actor Object Reference") (OtherComp :type "PrimitiveComponent Object Reference") (OtherBodyIndex :type Integer))
  (cast `/Game/Variant_Shooter/Blueprints/BP_ShooterCharacter` OtherActor)
  (set `self.Should rotate` false))

(fn `UserConstructionScript`)