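; Deprecated pickup actor that grants BP_ShooterCharacter a temporary speed boost.
; Sphere overlap while active plays a pickup sound, hides and deactivates the pickup, and doubles the character's max walk speed and sprint speed.
; Chained delays restore the cached original speeds, then make the pickup visible and active again after a cooldown.
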(event `self.Sphere.OnComponentBeginOverlap`
  (params (OverlappedComponent :type "PrimitiveComponent Object Reference") (OtherActor :type "Actor Object Reference") (OtherComp :type "PrimitiveComponent Object Reference") (OtherBodyIndex :type Integer) (bFromSweep :type Boolean) (SweepResult :type "HitResult Structure (by ref)"))
  (if (`self.bIsActive`)
    (if (== (`GameplayStatics.GetObjectClass` OtherActor) "/Game/Variant_Shooter/Blueprints/BP_ShooterCharacter.BP_ShooterCharacter_C")
      (`AudioComponent.Play` (`self.MS_SFX_Powerup_Pickup`) 0.0)
      (bind _asbp_shooter_character (cast `/Game/Variant_Shooter/Blueprints/BP_ShooterCharacter` OtherActor))
      (set `self.bIsActive` false)
      (bind _charactermovement (`Character.CharacterMovement` _asbp_shooter_character))
      (bind _output_get (set `self.StandardWalkSpeed` (`CharacterMovementComponent.MaxWalkSpeed` _charactermovement)))
      (bind _output_get_2 (set `self.UpgradedSprintSpeed` (* _output_get 2.0)))
      (set `CharacterMovementComponent.MaxWalkSpeed` _output_get_2 _charactermovement)
      (bind _output_get_3 (set `self.StandardSprintSpeed` (`/Game/Variant_Shooter/Blueprints/BP_ShooterCharacter.Sprint Speed` _asbp_shooter_character)))
      (bind _output_get_4 (set `self.UpgradedSprintSpeed` (* _output_get_3 2.0)))
      (set `/Game/Variant_Shooter/Blueprints/BP_ShooterCharacter.Sprint Speed` _output_get_4 _asbp_shooter_character)
      (`SceneComponent.SetVisibility` (`self.DefaultSceneRoot`) false true)
      (`KismetSystemLibrary.Delay` 10.0)
      (set `/Game/Variant_Shooter/Blueprints/BP_ShooterCharacter.Sprint Speed` (`self.StandardSprintSpeed`) _asbp_shooter_character)
      (set `CharacterMovementComponent.MaxWalkSpeed` (`self.StandardWalkSpeed`) _charactermovement)
      (`KismetSystemLibrary.Delay` 10.0)
      (set `self.bIsActive` true)
      (`SceneComponent.SetVisibility` (`self.DefaultSceneRoot`) true true))))

(fn `UserConstructionScript`)