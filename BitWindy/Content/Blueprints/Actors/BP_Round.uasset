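; BP_Round is a timed round actor that counts down either a combat round or a between-round wait.
; Start sets limits and a looping 0.01-second timer, capped at once per frame, as a custom tick.
; Each tick broadcasts remaining time, then either dispatches spawn intervals or, at zero, RoundTimerDone without clearing the timer.
; Only combat rounds bind the spawn dispatcher to BP_EnemySpawnerManager, so waits spawn nothing through it.
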(event `RoundTick`
  ; Custom frame rate safe tick
  (`self.HandleRoundTick` (`KismetSystemLibrary.K2_GetTimerElapsedTimeHandle` (`self.RoundTimer`))))

(fn `End`
  (`self.RoundTimerDone`))

(fn `HandleEnemySpawnIntervalCalc`
  (params (RoundDeltaTime :type "Float (double-precision)"))
  ; If it has been SpawnFrequency seconds since last spawn event dispatch, call it and reset the interval tracker
  (bind _output_get (set `self.TimeSinceLastSpawn` (+ (`self.TimeSinceLastSpawn`) RoundDeltaTime)))
  (if (>= _output_get (`self.SpawnFrequency`))
    (`self.EnemySpawnIntervalReached`)
    (set `self.TimeSinceLastSpawn` 0.0)))

(fn `HandleRoundTick`
  (params (RoundDeltaTime :type "Float (double-precision)"))
  ; Decrement the amount of time left in the round and then notify of new time
  (bind _output_get (set `self.TimeRemaining` (- (`self.TimeRemaining`) RoundDeltaTime)))
  (`self.RoundTimeTick` _output_get (`self.bBetweenRound`))
  ; if no time remains, end the round
  (if (<= (`self.TimeRemaining`) 0.0)
    (`self.End`)
    (else
      ; if Round is still going, see if the enemy spawn interval has been reached
      (`self.HandleEnemySpawnIntervalCalc` (`local.RoundDeltaTime`)))))

(fn `HandleSignalConnection`
  (if (not (`self.bBetweenRound`))
    ; Set up enemy spawn timing logic via the manager
    (bind _returnvalue (`GameplayStatics.GetActorOfClass` "/Game/Blueprints/Actors/BP_EnemySpawnerManager.BP_EnemySpawnerManager_C"))
    (add `self.EnemySpawnIntervalReached` (`|CreateDelegate` _returnvalue :!event `OnEnemySpawnIntervalReached`))))

(fn `HandleTimerInitialization`
  ; Set up enemies to start spawning immediately
  (set `self.TimeSinceLastSpawn` (`self.SpawnFrequency`))
  ; Keep reference to Timer for clearing on End()
  (bind _returnvalue (`KismetSystemLibrary.K2_SetTimerDelegate` (`|CreateDelegate` :!event `RoundTick`) 0.01 true true))
  (set `self.RoundTimer` _returnvalue))

(fn `OnRep_RoundTimer`)

(fn `PrintTimeRemaining`
  (params (TimeRemaining :type "Float (double-precision)"))
  (locals (PrintTimeRemaining :type String))
  (if (`self.bBetweenRound`)
    (`KismetSystemLibrary.PrintString` (`KismetStringLibrary.Concat_StrStr` "Time Remaining in Wait Round: " (`KismetStringLibrary.TimeSecondsToString` TimeRemaining)) true false (struct :`R` 0.032141 :`G` 1.0 :`A` 1.0) 5.0 "RoundTimerDisplay")
    (else
      (`KismetSystemLibrary.PrintString` (`KismetStringLibrary.Concat_StrStr` "Time Remaining in Combat Round: " (`KismetStringLibrary.TimeSecondsToString` TimeRemaining)) true false (struct :`R` 1.0 :`G` 0.179111 :`A` 1.0) 5.0 "RoundTimerDisplay"))))

(fn `Start`
  (params (`Round Time Limit` :type "Float (double-precision)") (`Round Spawn Frequency` :type "Float (double-precision)") (bBetweenRound :type Boolean))
  ; variable initialization
  (bind _output_get (set `self.TimeLimit` `Round Time Limit`))
  (set `self.TimeRemaining` _output_get)
  (set `self.SpawnFrequency` `Round Spawn Frequency`)
  (set `self.bBetweenRound` bBetweenRound)
  (`self.HandleSignalConnection`)
  (`self.HandleTimerInitialization`))

(fn `UserConstructionScript`
  (`self.HandleSignalConnection`))