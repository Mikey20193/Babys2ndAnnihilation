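; Speed boost pickup that temporarily multiplies a player's walk and sprint speeds, built on a parent powerup class.
; The ApplyPowerup override saves the current speeds, applies Multiplier through SetPlayerMovement, then calls the parent implementation.
; It hands the saved speeds to an EventGraph event, which waits PowerUpTime before restoring them, keeping the latent Delay out of the function.
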(event `DelayThenResetPlayer`
  (params (Player :type "/Game/Variant_Shooter/Blueprints/BP_ShooterCharacter Object Reference") (BaseWalk :type "Float (double-precision)") (BaseSprint :type "Float (double-precision)"))
  (`KismetSystemLibrary.Delay` (`self.Power Up time`))
  (`self.SetPlayerMovement` Player BaseWalk BaseSprint))

(fn `ApplyPowerup`
  (params (Player :type "/Game/Variant_Shooter/Blueprints/BP_ShooterCharacter Object Reference"))
  (locals (BaseSprint :type "Float (double-precision)") (BaseWalk :type "Float (double-precision)"))
  (bind _player (`local.Player`))
  (bind _output_get (set `local.BaseSprint` (`/Game/Variant_Shooter/Blueprints/BP_ShooterCharacter.Sprint Speed` Player)))
  (bind _output_get_2 (set `local.BaseWalk` (`CharacterMovementComponent.MaxWalkSpeed` (`Character.CharacterMovement` Player))))
  (`self.SetPlayerMovement` _player (* _output_get_2 (`self.Multiplier`)) (* _output_get (`self.Multiplier`)))
  (`parent.ApplyPowerup` _player)
  (`self.DelayThenResetPlayer` _player (`local.BaseWalk`) (`local.BaseSprint`)))

(fn `SetPlayerMovement`
  (params (Player :type "/Game/Variant_Shooter/Blueprints/BP_ShooterCharacter Object Reference") (Walk :type "Float (double-precision)") (Sprint :type "Float (double-precision)"))
  (set `CharacterMovementComponent.MaxWalkSpeed` Walk (`Character.CharacterMovement` Player))
  (set `/Game/Variant_Shooter/Blueprints/BP_ShooterCharacter.Sprint Speed` Sprint Player))

(fn `UserConstructionScript`
  (`parent.UserConstructionScript`))