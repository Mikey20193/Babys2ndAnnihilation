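; BP_Tower_Domination is a capture-point tower that scores for the team with more characters in its sphere, and can also be destroyed.
; Overlaps fill per-team arrays with team indices rather than players, compared on overlap changes and via a delayed Tick to award game-state points.
; Damage from anything but player snowballs lowers health and updates the indicator widget.
; At zero health, avalanche effects play and a timeline sinks tower and characters.
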(event `self.ReceiveTick`
  (params (DeltaSeconds :type "Float (single-precision)"))
  (`KismetSystemLibrary.Delay` 0.5)
  (`self.Check for score point`))

(event `self.ReceiveBeginPlay`
  (bind _returnvalue (`KismetMathLibrary.RandomFloatInRange` 0.0 2.5))
  (bind _tower_name (`self.Tower Name`))
  (`KismetSystemLibrary.Delay` 2.0)
  (bind _asbp_gs_koth (cast `/Game/Blueprints/GameArchitecture/GameModes/KOTH/BP_GS_KOTH` (`GameplayStatics.GetGameState`)))
  (set `self.As Game State` _asbp_gs_koth)
  (set `self.DomeLocation` (`SceneComponent.K2_GetComponentLocation` (`self.Dome`)))
  (`|PlayMontage` (`self.SK_Char_Friendly2`) "/Game/3D_Assets/Characters/Friendly/AM_Char_Friendly_Afraid.AM_Char_Friendly_Afraid" 0.7 _returnvalue
    (:`then`
      (`|PlayMontage` (`self.SK_Char_Friendly1`) "/Game/3D_Assets/Characters/Friendly/AM_Char_Friendly_Afraid.AM_Char_Friendly_Afraid" 0.7 _returnvalue
        (:`then`
          (bind _aswb_tower_indicator (cast `/Game/Variant_Shooter/UI/WB_TowerIndicator` (`WidgetComponent.GetWidget` (`self.TowerUI`))))
          (bind _output_get (set `self.WB Tower Indicator` _aswb_tower_indicator))
          (switch `/Game/Data/ETower` _tower_name
            (:`NewEnumerator0`
              (set `/Game/Variant_Shooter/UI/WB_TowerIndicator.Tower Name` "★" _output_get))
            (:`NewEnumerator1`
              (set `/Game/Variant_Shooter/UI/WB_TowerIndicator.Tower Name` (`KismetTextLibrary.Conv_StringToText` (`KismetStringLibrary.RightChop` (`|GetEnumeratorNameAsString` _tower_name) 5)) _output_get :!label _label))
            (:`NewEnumerator2`
              (goto _label))
            (:`NewEnumerator3`
              (goto _label)))
          (`self.TowerUIBillboard`)
          (add `self.TowerDestroyed` (`|CreateDelegate` :!event `OnTowerDestroyed`)))))))

(event `self.DoDamage`
  (params (Damage :type "Float (double-precision)") (HitProjectile :type "StaticMeshComponent Object Reference") (`Damage Causer` :type "/Game/Variant_Shooter/Blueprints/BP_ShooterCharacter Object Reference"))
  (if (`KismetSystemLibrary.IsValid` HitProjectile)
    (if (not (`ActorComponent.ComponentHasTag` HitProjectile "PlayerSnowball"))
      (`self.TakeDamage` Damage :!label _label_2))
    (else
      (goto _label_2))))

(event `OnTowerDestroyed`
  (bind _sk_char_friendly1 (`self.SK_Char_Friendly1`))
  (bind _sk_char_friendly2 (`self.SK_Char_Friendly2`))
  (`NiagaraFunctionLibrary.SpawnSystemAtLocation` "/Game/VFX/N_Avalanch.N_Avalanch" (+ (`self.DomeLocation`) (0.0 0.0 200.0)))
  (`AudioComponent.Play` (`self.Tower_Destroyed`) 0.0)
  (bind (_direction _newtrack_0) (`Timeline|Timeline` :`NewTime` 1.0)
    (:`Update`
      (bind _returnvalue (* _newtrack_0 320.0))
      (`SceneComponent.K2_SetWorldLocation` (`self.Tower`) (- (`self.DomeLocation`) (`KismetMathLibrary.MakeVector` 0.0 0.0 _returnvalue)) false false)
      (`SceneComponent.K2_SetWorldLocation` _sk_char_friendly1 (- (`SceneComponent.K2_GetComponentLocation` _sk_char_friendly1) (`KismetMathLibrary.MakeVector` 0.0 0.0 _returnvalue)) false false)
      (`SceneComponent.K2_SetWorldLocation` _sk_char_friendly2 (- (`SceneComponent.K2_GetComponentLocation` _sk_char_friendly2) (`KismetMathLibrary.MakeVector` 0.0 0.0 _returnvalue)) false false))))

(event `Check for score point`
  (if (> (`KismetArrayLibrary.Array_Length` (`self.Team A Array`)) (`KismetArrayLibrary.Array_Length` (`self.Team B Array`)))
    (`/Game/Blueprints/GameArchitecture/GameModes/KOTH/BP_GS_KOTH.Add Score Team A` (`self.As Game State`))
    (elif (> (`KismetArrayLibrary.Array_Length` (`self.Team B Array`)) (`KismetArrayLibrary.Array_Length` (`self.Team A Array`)))
      (`/Game/Blueprints/GameArchitecture/GameModes/KOTH/BP_GS_KOTH.Add Score Team B` (`self.As Game State`)))))

(event `self.Sphere.OnComponentBeginOverlap`
  (params (OverlappedComponent :type "PrimitiveComponent Object Reference") (OtherActor :type "Actor Object Reference") (OtherComp :type "PrimitiveComponent Object Reference") (OtherBodyIndex :type Integer) (bFromSweep :type Boolean) (SweepResult :type "HitResult Structure (by ref)"))
  (bind _asbp_shooter_character (cast `/Game/Variant_Shooter/Blueprints/BP_ShooterCharacter` OtherActor))
  (bind _asbp_ps_koth (cast `/Game/Blueprints/GameArchitecture/GameModes/KOTH/BP_PS_KOTH` (`Pawn.PlayerState` _asbp_shooter_character)))
  (bind _team_index (`/Game/Blueprints/GameArchitecture/GameModes/KOTH/BP_PS_KOTH.Team Index` _asbp_ps_koth))
  (switch `int` _team_index
    (:`0`
      (`KismetArrayLibrary.Array_Add` (`self.Team A Array`) _team_index))
    (:`1`
      (`KismetArrayLibrary.Array_Add` (`self.Team B Array`) _team_index)))
  (`self.Check for score point`))

(event `self.Sphere.OnComponentEndOverlap`
  (params (OverlappedComponent :type "PrimitiveComponent Object Reference") (OtherActor :type "Actor Object Reference") (OtherComp :type "PrimitiveComponent Object Reference") (OtherBodyIndex :type Integer))
  (bind _asbp_shooter_character (cast `/Game/Variant_Shooter/Blueprints/BP_ShooterCharacter` OtherActor))
  (bind _asbp_ps_koth (cast `/Game/Blueprints/GameArchitecture/GameModes/KOTH/BP_PS_KOTH` (`Pawn.PlayerState` _asbp_shooter_character)))
  (bind _team_index (`/Game/Blueprints/GameArchitecture/GameModes/KOTH/BP_PS_KOTH.Team Index` _asbp_ps_koth))
  (switch `int` _team_index
    (:`0`
      (`KismetArrayLibrary.Array_RemoveItem` (`self.Team A Array`) _team_index))
    (:`1`
      (`KismetArrayLibrary.Array_RemoveItem` (`self.Team B Array`) _team_index)))
  (`self.Check for score point`))

(fn `CheckObjectHealth`
  (returns (Health :type "Float (double-precision)"))
  (return (`self.CurrentHealth`)))

(fn `DestroyTower`
  (set `self.bTowerDestroyed` true)
  (`self.Update UI after Destroyed`)
  (`ActorComponent.K2_DestroyComponent` (`self.Cutout_from_dome`))
  (`ActorComponent.K2_DestroyComponent` (`self.Cutout_from_tower`))
  (`self.TowerDestroyed`))

(fn `TakeDamage`
  (params (`Damage Amount` :type "Float (double-precision)"))
  (if (not (`self.bTowerDestroyed`))
    (`/Game/Variant_Shooter/UI/WB_TowerIndicator.PlayUnderAttackAnim` (`self.WB Tower Indicator`))
    (bind _output_get (set `self.CurrentHealth` (`KismetMathLibrary.FClamp` (- (`self.CurrentHealth`) `Damage Amount`) 0.0 (`self.MaxHealth`))))
    (`self.TowerHealthChanged` _output_get (`self.MaxHealth`) (`self.Tower Name`))
    (if (== (`self.CurrentHealth`) 0.0)
      (`self.DestroyTower`))))

(fn `TowerUIBillboard`)

(fn `Update UI after Destroyed`
  (bind _wb_tower_indicator (`self.WB Tower Indicator`))
  (`Image.SetBrushFromTexture` (`/Game/Variant_Shooter/UI/WB_TowerIndicator.TowerImage` _wb_tower_indicator) (`/Game/Variant_Shooter/UI/WB_TowerIndicator.TowerDestroyedImage` _wb_tower_indicator) false)
  (set `TextBlock.Text` "" (`/Game/Variant_Shooter/UI/WB_TowerIndicator.TextBlock_26` _wb_tower_indicator)))

(fn `UserConstructionScript`)