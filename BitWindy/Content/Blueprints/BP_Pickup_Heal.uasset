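; BP_Pickup_Heal is a healing pickup that restores health to the player who receives it.
; It overrides ApplyPowerup to add HealAmount to the player's current HP, clamped between zero and max HP.
; It then pushes the new value to the health UI through the player controller before calling the parent implementation.
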(fn `ApplyPowerup`
  (params (Player :type "/Game/Variant_Shooter/Blueprints/BP_ShooterCharacter Object Reference"))
  (bind _output_get (set `/Game/Variant_Shooter/Blueprints/BP_ShooterCharacter.Current HP` (`KismetMathLibrary.FClamp` (+ (`/Game/Variant_Shooter/Blueprints/BP_ShooterCharacter.Current HP` Player) (`self.HealAmount`)) 0.0 (`/Game/Variant_Shooter/Blueprints/BP_ShooterCharacter.Max HP` Player)) Player))
  (message `/Game/Variant_Shooter/Blueprints/BPI_Shooter.Update Health UI` (`/Game/Variant_Shooter/Blueprints/BP_ShooterCharacter.Player Controller` Player) _output_get)
  (`parent.ApplyPowerup` Player))

(fn `UserConstructionScript`
  (`parent.UserConstructionScript`))