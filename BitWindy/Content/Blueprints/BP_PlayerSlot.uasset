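; BP_PlayerSlot is a lobby podium slot that shows a shooter character for the player assigned to it.
; AddPlayer stores the controller, replaces any existing character with a new BP_ShooterCharacter at the Arrow's transform, and lifts it by the capsule half-height.
; It then passes the Arrow's transform to BP_LobbyController as the current podium transform.
; RemovePlayer clears the controller and destroys the character.
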(event `Add Player`
  (params (PC :type "PlayerController Object Reference"))
  (bind _returnvalue (`SceneComponent.K2_GetComponentToWorld` (`self.Arrow`)))
  (set `self.PC` PC)
  (bind _selected_charatcer (`self.Selected Charatcer`)
    (:`then`
      (`self.K2_DestroyActor` _selected_charatcer))
    (:`else`
      _))
  (bind _returnvalue_2 (`|SpawnActorFromClass` "/Game/Variant_Shooter/Blueprints/BP_ShooterCharacter.BP_ShooterCharacter_C" (`SceneComponent.K2_GetComponentToWorld` (`self.Arrow`)) "AlwaysSpawn" "MultiplyWithRoot" null null))
  (bind _output_get (set `self.Selected Charatcer` _returnvalue_2))
  (`self.K2_SetActorTransform` _output_get (`KismetMathLibrary.MakeTransform` (`KismetMathLibrary.MakeVector` (.x (.location _returnvalue)) (.y (.location _returnvalue)) (+ (`CapsuleComponent.GetScaledCapsuleHalfHeight` (`Character.CapsuleComponent` _returnvalue_2)) (.z (.location _returnvalue)))) (.rotation _returnvalue) (.scale _returnvalue)) false false)
  (bind _asbp_lobby_controller (cast `/Game/Blueprints/BP_LobbyController` (`self.PC`)))
  (`/Game/Blueprints/BP_LobbyController.SetCurrentPodiumTransform` _asbp_lobby_controller (`SceneComponent.K2_GetComponentToWorld` (`self.Arrow`))))

(event `Remove Player`
  (set `self.PC` null)
  (bind _selected_charatcer (`self.Selected Charatcer`)
    (:`then`
      (`self.K2_DestroyActor` _selected_charatcer)
      (set `self.Selected Charatcer` null))
    (:`else`)))

(fn `UserConstructionScript`)