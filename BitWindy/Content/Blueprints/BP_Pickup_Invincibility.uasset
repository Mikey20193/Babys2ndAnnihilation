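; Pickup actor that, despite its Invincibility name, temporarily switches an overlapping BP_ShooterCharacter's weapon to the rifle.
; Sphere overlap deactivates and hides the pickup, then sets the character's weapon class and refreshes the equipped weapon.
; After a delay it clears the character's owned weapons and equips the grenade launcher.
; A second delay in the same chain then reactivates and shows the pickup for reuse.
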(event `self.Sphere.OnComponentBeginOverlap`
  (params (OverlappedComponent :type "PrimitiveComponent Object Reference") (OtherActor :type "Actor Object Reference") (OtherComp :type "PrimitiveComponent Object Reference") (OtherBodyIndex :type Integer) (bFromSweep :type Boolean) (SweepResult :type "HitResult Structure (by ref)"))
  (if (`self.bIsActive`)
    (if (== (`GameplayStatics.GetObjectClass` OtherActor) "/Game/Variant_Shooter/Blueprints/BP_ShooterCharacter.BP_ShooterCharacter_C")
      (bind _asbp_shooter_character (cast `/Game/Variant_Shooter/Blueprints/BP_ShooterCharacter` OtherActor))
      (set `self.bIsActive` false)
      (set `/Game/Variant_Shooter/Blueprints/BP_ShooterCharacter.Weapon Class` "/Game/Variant_Shooter/Blueprints/Pickups/Weapons/BP_ShooterWeapon_Rifle.BP_ShooterWeapon_Rifle_C" _asbp_shooter_character)
      (`/Game/Variant_Shooter/Blueprints/BP_ShooterCharacter.Update Equiped Weapon` _asbp_shooter_character)
      (`SceneComponent.SetVisibility` (`self.DefaultSceneRoot`) false true)
      (`KismetSystemLibrary.Delay` 10.0)
      (`KismetArrayLibrary.Array_Clear` (`/Game/Variant_Shooter/Blueprints/BP_ShooterCharacter.Owned Weapons` _asbp_shooter_character))
      (set `/Game/Variant_Shooter/Blueprints/BP_ShooterCharacter.Weapon Class` "/Game/Variant_Shooter/Blueprints/Pickups/Weapons/BP_ShooterWeapon_GrenadeLauncher.BP_ShooterWeapon_GrenadeLauncher_C" _asbp_shooter_character)
      (`/Game/Variant_Shooter/Blueprints/BP_ShooterCharacter.Update Equiped Weapon` _asbp_shooter_character)
      (`KismetSystemLibrary.Delay` 10.0)
      (set `self.bIsActive` true)
      (`SceneComponent.SetVisibility` (`self.DefaultSceneRoot`) true true))))

(fn `UserConstructionScript`)