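; Fire-rate pickup Blueprint that temporarily swaps a player's grenade launcher for the rifle.
; ApplyPowerup changes the weapon class and refreshes the equipped weapon only if the player has the grenade launcher, then runs the parent logic.
; In that case it also triggers ResetPowerup, which waits for Duration, clears owned weapons and re-equips the grenade launcher.
; Players with any other weapon receive only the parent powerup behavior.
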(event `ResetPowerup`
  (params (Player :type "/Game/Variant_Shooter/Blueprints/BP_ShooterCharacter Object Reference"))
  (`KismetSystemLibrary.Delay` (`self.Duration`))
  (`KismetArrayLibrary.Array_Clear` (`/Game/Variant_Shooter/Blueprints/BP_ShooterCharacter.Owned Weapons` Player))
  (set `/Game/Variant_Shooter/Blueprints/BP_ShooterCharacter.Weapon Class` "/Game/Variant_Shooter/Blueprints/Pickups/Weapons/BP_ShooterWeapon_GrenadeLauncher.BP_ShooterWeapon_GrenadeLauncher_C" Player)
  (`/Game/Variant_Shooter/Blueprints/BP_ShooterCharacter.Update Equiped Weapon` Player))

(fn `ApplyPowerup`
  (params (Player :type "/Game/Variant_Shooter/Blueprints/BP_ShooterCharacter Object Reference"))
  (if (== (`/Game/Variant_Shooter/Blueprints/BP_ShooterCharacter.Weapon Class` Player) "/Game/Variant_Shooter/Blueprints/Pickups/Weapons/BP_ShooterWeapon_GrenadeLauncher.BP_ShooterWeapon_GrenadeLauncher_C")
    (set `/Game/Variant_Shooter/Blueprints/BP_ShooterCharacter.Weapon Class` "/Game/Variant_Shooter/Blueprints/Pickups/Weapons/BP_ShooterWeapon_Rifle.BP_ShooterWeapon_Rifle_C" Player)
    (`/Game/Variant_Shooter/Blueprints/BP_ShooterCharacter.Update Equiped Weapon` Player)
    (`parent.ApplyPowerup` Player)
    (`self.ResetPowerup` Player)
    (else
      (`parent.ApplyPowerup` Player))))

(fn `UserConstructionScript`
  (`parent.UserConstructionScript`))