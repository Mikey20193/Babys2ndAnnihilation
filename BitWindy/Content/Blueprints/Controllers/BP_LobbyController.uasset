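; Player controller for the lobby that shows the lobby screen and manages player info and ready status.
; Run-on-server events update player info and toggle readiness through the lobby game mode.
; Timelines lerp the lobby pawn toward the current podium and back to its saved transform.
; In tower defense levels it spawns a shooter controller, transfers player state ownership, controller ID and pawn, then destroys itself.
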(event `Look Away from Podium`
  (bind _lobby_ui (`self.Lobby ui`))
  ; Camera Lerping Events
  (bind _asbp_lobby_controller (cast `/Game/Blueprints/Controllers/BP_LobbyController` (`GameplayStatics.GetPlayerController` 0)))
  (bind _asbp_lobby_pawn (cast `/Game/Blueprints/Controllers/BP_LobbyPawn` (`self.K2_GetPawn` _asbp_lobby_controller)))
  (`Widget.SetVisibility` (`self.Lobby ui`) "Visible")
  (`Widget.SetVisibility` (`/Game/UI/Widgets/Screens/WB_LobbyScreen.DisplayContainer` (`self.Lobby ui`)) "Hidden")
  (`Widget.SetVisibility` (`/Game/UI/Widgets/Screens/WB_LobbyScreen.Image_Background` (`self.Lobby ui`)) "Hidden")
  (`UserWidget.PlayAnimation` _lobby_ui (`/Game/UI/Widgets/Screens/WB_LobbyScreen.ShowReadyStartMenu` _lobby_ui) 0.0 1 "Forward" 1.0 false)
  (bind (_direction _newtrack_0) (`Timeline|Timeline_0` :!via `PlayFromStart`)
    (:`Update`
      (bind (_returnvalue_location _returnvalue_rotation) (`KismetMathLibrary.BreakTransform` (`KismetMathLibrary.TLerp` (`self.GetTransform` _asbp_lobby_pawn) (`self.Starting Transform`) _newtrack_0)))
      (`self.K2_SetActorLocationAndRotation` _asbp_lobby_pawn _returnvalue_location _returnvalue_rotation false false))))

(event `Look At Podium`
  ; Camera Lerping Events
  (bind _asbp_lobby_controller (cast `/Game/Blueprints/Controllers/BP_LobbyController` (`GameplayStatics.GetPlayerController` 0)))
  (bind _asbp_lobby_pawn (cast `/Game/Blueprints/Controllers/BP_LobbyPawn` (`self.K2_GetPawn` _asbp_lobby_controller)))
  (set `self.Starting Transform` (`self.GetTransform` _asbp_lobby_pawn))
  (bind (_direction _newtrack_0) (`Timeline|Timeline` :!via `PlayFromStart`)
    (:`Update`
      (bind _current_podium (`/Game/Blueprints/Controllers/BP_LobbyController.Current Podium` _asbp_lobby_controller))
      (bind _returnvalue_location (`KismetMathLibrary.BreakTransform` (`self.GetTransform` _asbp_lobby_pawn)))
      (bind (_returnvalue_location_2 _returnvalue_rotation) (`KismetMathLibrary.BreakTransform` (`KismetMathLibrary.TLerp` (`self.Starting Transform`) (`KismetMathLibrary.MakeTransform` (- (`KismetMathLibrary.MakeVector` (.x (.location _current_podium)) (.y (.location _current_podium)) (.z (.location _current_podium))) (400.0 -50.0 -50.0)) (`KismetMathLibrary.FindLookAtRotation` _returnvalue_location (`KismetMathLibrary.MakeVector` (.x (.location _current_podium)) (.y (.location _current_podium)) (+ (.z (.location _current_podium)) 100.0)))) _newtrack_0)))
      (`self.K2_SetActorLocationAndRotation` _asbp_lobby_pawn _returnvalue_location_2 _returnvalue_rotation false false))))

(event `SwitchToShooterController`
  (bind _returnvalue (`self.K2_GetPawn`))
  (bind _new_controller (`self.New Controller`))
  ; Function to switch to shooter controller
  (`KismetSystemLibrary.Delay` 0.5)
  (set `self.Player State` (`GameplayStatics.GetPlayerState` 0))
  (set `self.OldPawn` _returnvalue)
  (bind _returnvalue_2 (`|SpawnActorFromClass` "/Game/Variant_Shooter/Blueprints/BP_ShooterPlayerController.BP_ShooterPlayerController_C" (`self.GetTransform` _returnvalue) "Undefined" "MultiplyWithRoot" null null null))
  (bind _output_get (set `self.New Controller` _returnvalue_2))
  (`self.SetOwner` (`self.Player State`) _output_get)
  (`GameplayStatics.SetPlayerControllerID` _new_controller (`GameplayStatics.GetPlayerControllerID` self))
  (`self.Possess` _new_controller (`self.OldPawn`))
  (`KismetSystemLibrary.RaiseScriptError` "Switched to Lobby")
  (`self.K2_DestroyActor` self))

(event `Update Player Info`
  ; Player Info Controls and replication
  (`KismetSystemLibrary.Delay` 0.1)
  (`self.ROS_UpdatePlayerInfo`))

(event `ROS_UpdatePlayerInfo`
  ; Player Info Controls and replication
  (bind _asbp_lobby_game_mode (cast `/Game/Blueprints/GameArchitecture/GameModes/BP_Lobby_GameMode` (`GameplayStatics.GetGameMode`)))
  (`/Game/Blueprints/GameArchitecture/GameModes/BP_Lobby_GameMode.Update Player Info` _asbp_lobby_game_mode self))

(event `ROS_ToggleReadyStatus`
  (bind _player_info (`self.Player Info`))
  ; Player Info Controls and replication
  (setmembers `/Game/Blueprints/S_PlayerInfo` :`StructRef` _player_info :`Ready` (not (`.Ready_13_EFEBA9314AB0A2B53DD1EDA942A324FB` (break `/Game/Blueprints/S_PlayerInfo` _player_info))))
  (bind _asbp_lobby_game_mode (cast `/Game/Blueprints/GameArchitecture/GameModes/BP_Lobby_GameMode` (`GameplayStatics.GetGameMode`)))
  (`/Game/Blueprints/GameArchitecture/GameModes/BP_Lobby_GameMode.Update Player Info` _asbp_lobby_game_mode self))

(event `self.ReceiveBeginPlay`
  ; Begin Play function
  (set `self.OldPawn` null)
  (set `self.New Controller` null)
  (set `self.Lobby ui` null)
  (cast `/Game/Blueprints/Controllers/BP_LobbyController` (`GameplayStatics.GetPlayerController` 0))
  (bind _returnvalue (`GameplayStatics.GetCurrentLevelName` true))
  (if (`KismetStringLibrary.Contains` _returnvalue "LV_TowerDefense")
    (`KismetSystemLibrary.Delay` 0.5)
    (`self.SwitchToShooterController`)
    (elif (`self.IsLocalPlayerController`)
      (bind _returnvalue_2 (`|CreateWidget` "/Game/UI/Widgets/Screens/WB_LobbyScreen.WB_LobbyScreen_C"))
      (bind _output_get (set `self.Lobby ui` _returnvalue_2))
      (`UserWidget.AddToViewport` _output_get 0)
      (set `self.bShowMouseCursor` true)
      (`WidgetBlueprintLibrary.SetInputMode_GameAndUIEx` self (`self.Lobby ui`))
      (`self.ROS_UpdatePlayerInfo`))))

(fn `SetCurrentPodiumTransform`
  (params (CurrentPodium :type "Transform Structure"))
  (set `self.Current Podium` CurrentPodium))

(fn `UserConstructionScript`)