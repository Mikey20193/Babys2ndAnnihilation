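; BP_LobbyController is the lobby player controller that gives the local player a lobby screen and reports their player info.
; On BeginPlay, the local controller creates WB_LobbyScreen, enables the cursor with Game and UI input, and requests an info update.
; ROS events pass the controller to BP_LobbyGameMode, either to refresh info or after toggling Ready in PlayerInfo.
; UpdatePlayerInfo repeats the refresh request after a short delay.
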(event `self.ReceiveBeginPlay`
  (if (`self.IsLocalPlayerController`)
    (bind _returnvalue (`|CreateWidget` "/Game/UI/Widgets/WB_LobbyScreen.WB_LobbyScreen_C"))
    (bind _output_get (set `self.Lobby ui` _returnvalue))
    (`UserWidget.AddToViewport` _output_get 0)
    (set `self.bShowMouseCursor` true)
    (`WidgetBlueprintLibrary.SetInputMode_GameAndUIEx` self (`self.Lobby ui`))
    (`self.ROS_UpdatePlayerInfo`)))

(event `Update Player Info`
  (`KismetSystemLibrary.Delay` 0.1)
  (`self.ROS_UpdatePlayerInfo`))

(event `ROS_UpdatePlayerInfo`
  (bind _asbp_lobby_game_mode (cast `/Game/Blueprints/GameArchitecture/BP_LobbyGameMode` (`GameplayStatics.GetGameMode`)))
  (`/Game/Blueprints/GameArchitecture/BP_LobbyGameMode.Update Player Info` _asbp_lobby_game_mode self))

(event `ROS_ToggleReadyStatus`
  (bind _player_info (`self.Player Info`))
  (setmembers `/Game/Blueprints/S_PlayerInfo` :`StructRef` _player_info :`Ready` (not (`.Ready_13_EFEBA9314AB0A2B53DD1EDA942A324FB` (break `/Game/Blueprints/S_PlayerInfo` _player_info))))
  (bind _asbp_lobby_game_mode (cast `/Game/Blueprints/GameArchitecture/BP_LobbyGameMode` (`GameplayStatics.GetGameMode`)))
  (`/Game/Blueprints/GameArchitecture/BP_LobbyGameMode.Update Player Info` _asbp_lobby_game_mode self))

(fn `UserConstructionScript`)