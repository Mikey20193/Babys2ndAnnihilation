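; Player state for the free-for-all game mode that tracks each player's kills, deaths, match score and display name.
; AddKill raises the kill count and adds a per-kill score, while AddDeath raises the death count, each printing debug totals.
; Every change fires a score-values-changed dispatcher, and GetScores returns all four values at once.
; The player name is cached as text at BeginPlay.
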(event `self.ReceiveBeginPlay`
  (set `self.Player Name` (`KismetTextLibrary.Conv_StringToText` (`self.GetPlayerName`))))

(fn `Add Score`
  (bind _output_get (set `self.Match Score` (+ (`self.Match Score`) (`self.ScorePerKill`))))
  (`KismetSystemLibrary.PrintString` (`KismetStringLibrary.Concat_StrStr` "Player Score: " (`KismetStringLibrary.Conv_IntToString` _output_get)))
  (`self.OnScoreValuesChanged` self))

(fn `AddDeath`
  (bind _result (`/Engine/EditorBlueprintResources/StandardMacros.IncrementInt` (`self.Deaths`))
    (:`  `
      (bind _output_get (set `self.Deaths` _result))
      (`KismetSystemLibrary.PrintString` (`KismetStringLibrary.Concat_StrStr` "Player Deaths: " (`KismetStringLibrary.Conv_IntToString` _output_get)))
      (`self.OnScoreValuesChanged` self))))

(fn `AddKill`
  (bind _result (`/Engine/EditorBlueprintResources/StandardMacros.IncrementInt` (`self.Kills`))
    (:`  `
      (bind _output_get (set `self.Kills` _result))
      (`KismetSystemLibrary.PrintString` (`KismetStringLibrary.Concat_StrStr` "Player Kills: " (`KismetStringLibrary.Conv_IntToString` _output_get)))
      (`self.Add Score`)
      (`self.OnScoreValuesChanged` self))))

(fn `Get Scores`
  (returns (Kills :type Integer) (`Match Score` :type Integer) (Deaths :type Integer) (`Player Name` :type Text))
  (return (`self.Kills`) (`self.Match Score`) (`self.Deaths`) (`self.Player Name`)))

(fn `UserConstructionScript`)