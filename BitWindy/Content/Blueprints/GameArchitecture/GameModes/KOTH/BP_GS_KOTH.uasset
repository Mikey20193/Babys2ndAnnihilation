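; Game state for the King of the Hill mode, tracking both team scores, round number, match progress and winner.
; Score setters fire change dispatchers, and score RepNotifies refresh each player controller's KOTH HUD.
; A round-begin callback from the Round Manager updates round number and between-round state.
; When the match stops and should end, the MatchInProgress RepNotify shows post-game UI once after a delay, gated by authority unless Winner is 2.
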(event `Add Post Game Flow UI`
  (bind _returnvalue (`GameplayStatics.GetPlayerController` 0))
  (`/Engine/EditorBlueprintResources/StandardMacros.DoOnce` false
    (:`Completed`
      (bind _asbp_shooter_player_controller (cast `/Game/Variant_Shooter/Blueprints/BP_ShooterPlayerController` _returnvalue))
      (`KismetSystemLibrary.PrintString` (`KismetStringLibrary.Concat_StrStr` "local winner value on player GS" (`KismetStringLibrary.Conv_IntToString` (`self.Winner`))))
      (bind _asbp_ps_koth (cast `/Game/Blueprints/GameArchitecture/GameModes/KOTH/BP_PS_KOTH` (`Controller.PlayerState` _returnvalue)))
      (`KismetSystemLibrary.PrintString` (`KismetStringLibrary.Concat_StrStr` "Local player team int: " (`KismetStringLibrary.Conv_IntToString` (`/Game/Blueprints/GameArchitecture/GameModes/KOTH/BP_PS_KOTH.Team Index` _asbp_ps_koth))))
      (`KismetSystemLibrary.Delay` 1.0)
      (`/Game/Variant_Shooter/Blueprints/BP_ShooterPlayerController.Add Post Game Flow UI` _asbp_shooter_player_controller (`self.Winner`)))))

(event `OnRoundBegin`
  (params (RoundNumber :type Integer) (TimeInRound :type "Float (double-precision)") (bBetweenRound :type Boolean))
  ; Listeners
  (set `self.CurrentRoundNumber` RoundNumber)
  (set `self.bWaitingForNextCombatRound` bBetweenRound))

(fn `Add Score Team A`
  (bind _result (`/Engine/EditorBlueprintResources/StandardMacros.IncrementInt` (`self.Team A Score`))
    (:`  `
      (set `self.Team A Score` _result)
      (`self.OnTeamAScoreChange`))))

(fn `Add Score Team B`
  (set `self.Team B Score` (+ (`self.Team B Score`) 1))
  (`self.OnTeamBScoreChanged`))

(fn `InitDifficulty`
  (params (DifficultySettings :type "/Game/Data/F_DifficultySettings Structure"))
  (set `self.TotalNumberOfRounds` (`.RoundsTotal_13_E8E21C214C75EC55D4F9F4876AE688B8` (break `/Game/Data/F_DifficultySettings` DifficultySettings)))
  (set `self.CurrentRoundNumber` 1))

(fn `OnRep_MatchInProgress?`
  (bind _winner (`self.Winner`))
  (if (`self.MatchInProgress?`)
    _
    (elif (`self.Should end Game`)
      (bind _asbp_ps_koth (cast `/Game/Blueprints/GameArchitecture/GameModes/KOTH/BP_PS_KOTH` (`Controller.PlayerState` (`GameplayStatics.GetPlayerController` 0))))
      (bind _asbp_shooter_player_controller (cast `/Game/Variant_Shooter/Blueprints/BP_ShooterPlayerController` (`PlayerState.GetPlayerController` _asbp_ps_koth)))
      (if (== _winner 2)
        (`self.Add Post Game Flow UI`)
        (elif (== (`/Game/Blueprints/GameArchitecture/GameModes/KOTH/BP_PS_KOTH.Team Index` _asbp_ps_koth) _winner)
          (bind _returnvalue (`self.HasAuthority` _asbp_shooter_player_controller))
          (if _returnvalue
            (`self.Add Post Game Flow UI`))
          (elif _returnvalue
            (`self.Add Post Game Flow UI`)))))))

(fn `OnRep_Team A Score`
  (for _array_element (`self.PlayerArray`)
    (bind _asbp_shooter_player_controller (cast `/Game/Variant_Shooter/Blueprints/BP_ShooterPlayerController` (`PlayerState.GetPlayerController` _array_element)))
    (`/Game/UI/Widgets/Screens/WB_HUD_Domination.update Scores` (`/Game/Variant_Shooter/Blueprints/BP_ShooterPlayerController.KOTH_HUD` _asbp_shooter_player_controller))))

(fn `OnRep_Team B Score`
  (for _array_element (`self.PlayerArray`)
    (bind _asbp_shooter_player_controller (cast `/Game/Variant_Shooter/Blueprints/BP_ShooterPlayerController` (`PlayerState.GetPlayerController` _array_element)))
    (`/Game/UI/Widgets/Screens/WB_HUD_Domination.update Scores` (`/Game/Variant_Shooter/Blueprints/BP_ShooterPlayerController.KOTH_HUD` _asbp_shooter_player_controller))))

(fn `SetMatchInProgress`
  (params (`Is Match In Progress?` :type Boolean))
  (set `self.MatchInProgress?` `Is Match In Progress?`))

(fn `SetWinner`
  (params (Winner :type Integer))
  (set `self.Winner` Winner))

(fn `UserConstructionScript`)