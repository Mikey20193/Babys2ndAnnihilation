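; Player state for the King of the Hill mode, tracking a player's kills, deaths, match score and team index.
; Each kill also adds the per-kill score, and stat changes fire a score-changed dispatcher alongside debug prints.
; The team index's RepNotify tints a valid shooter character pawn red for team 1, while team 0 only prints.
; An older per-slot material swap remains unconnected.
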(fn `Add Score`
  (bind _output_get (set `self.Match Score` (+ (`self.Match Score`) (`self.ScorePerKill`))))
  (`KismetSystemLibrary.PrintString` (`KismetStringLibrary.Concat_StrStr` "Player Score: " (`KismetStringLibrary.Conv_IntToString` _output_get)))
  (`self.OnScoreValuesChanged` self))

(fn `AddDeath`
  (bind _result (`/Engine/EditorBlueprintResources/StandardMacros.IncrementInt` (`self.Deaths`))
    (:`  `
      (bind _output_get (set `self.Deaths` _result))
      (`KismetSystemLibrary.PrintString` (`KismetStringLibrary.Concat_StrStr` "Player Deaths: " (`KismetStringLibrary.Conv_IntToString` _output_get)))
      (`self.OnScoreValuesChanged` self))))

(fn `AddKill`
  (bind _result (`/Engine/EditorBlueprintResources/StandardMacros.IncrementInt` (`self.Kills`))
    (:`  `
      (bind _output_get (set `self.Kills` _result))
      (`KismetSystemLibrary.PrintString` (`KismetStringLibrary.Concat_StrStr` "Player Kills: " (`KismetStringLibrary.Conv_IntToString` _output_get)))
      (`self.Add Score`)
      (`self.OnScoreValuesChanged` self))))

(fn `OnRep_Team Index`
  (bind _returnvalue (`self.GetPawn`))
  (bind _team_index (`self.Team Index`))
  (`/Engine/EditorBlueprintResources/StandardMacros.IsValid` _returnvalue
    (:`Is Valid`
      (bind _asbp_shooter_character (cast `/Game/Variant_Shooter/Blueprints/BP_ShooterCharacter` _returnvalue))
      (switch `int` _team_index
        (:`0`
          (`KismetSystemLibrary.PrintString` "Team 0"))
        (:`1`
          (`KismetSystemLibrary.PrintString` "team 1")
          (`/Game/Variant_Shooter/Blueprints/BP_ShooterCharacter.Set Team colour Red` _asbp_shooter_character _team_index))))))

(fn `Set Team`
  (params (`Team Index` :type Integer))
  (set `self.Team Index` `Team Index`))

(fn `UserConstructionScript`)