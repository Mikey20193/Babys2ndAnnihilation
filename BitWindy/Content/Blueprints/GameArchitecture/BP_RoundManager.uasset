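; Round manager for the tower defense game that alternates timed combat rounds with intermission periods and tracks the round number.
; Intermissions reuse the round object as a countdown with no enemies; when it ends, a new round starts with time limit and spawn frequency scaled linearly from difficulty settings.
; Combat round ends broadcast RoundOver, AdvanceRounds starts the next intermission, and Init binds HUD and GameState to round events.
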(event `HandleRound`
  (bind _timebetweenrounds (`self.TimeBetweenRounds`))
  (bind _currround (`self.CurrRound`))
  (add `/Game/Blueprints/Actors/BP_Round.RoundTimerDone` _currround (`|CreateDelegate` :!event `OnRoundEnd`))
  (`/Game/Blueprints/Actors/BP_Round.Start` _currround _timebetweenrounds (+ _timebetweenrounds 1.0) true)
  (bind _output_get (set `self.bBetweenRounds` true))
  (`self.RoundBegin` (`self.CurrentRoundNumber`) (`self.TimeBetweenRounds`) _output_get))

(event `OnRoundEnd`
  (`self.HandleRoundEnd`))

(fn `AdvanceRounds`
  (`/Engine/EditorBlueprintResources/StandardMacros.IncrementInt` (`self.CurrentRoundNumber`)
    (:`  `
      (`self.WaitForNextRound`))))

(fn `BeginNextRound`
  (bind (_timelimit _spawnfrequency) (`self.CalculateNextRoundTimerParameters`))
  (bind _asbp_adv_game_instance (cast `/Game/BitWindy/Multiplayer/BP_AdvGameInstance` (`GameplayStatics.GetGameInstance`)))
  (`/Game/BitWindy/Multiplayer/BP_AdvGameInstance.ROS_CreateRound` _asbp_adv_game_instance)
  (bind _current_round (`/Game/BitWindy/Multiplayer/BP_AdvGameInstance.Current Round` _asbp_adv_game_instance))
  (add `/Game/Blueprints/Actors/BP_Round.RoundTimerDone` _current_round (`|CreateDelegate` :!event `OnRoundEnd`))
  (`/Game/Blueprints/Actors/BP_Round.Start` _current_round _timelimit _spawnfrequency false)
  (set `self.CurrRound` _current_round)
  (bind _output_get (set `self.bBetweenRounds` false))
  (`self.RoundBegin` (`self.CurrentRoundNumber`) _timelimit _output_get))

(fn `CalculateNextRoundTimerParameters`
  (returns (TimeLimit :type "Float (double-precision)") (SpawnFrequency :type "Float (double-precision)"))
  (bind _returnvalue (- (`self.CurrentRoundNumber`) 1))
  (bind _returnvalue_2 (+ (`self.BaseTimeLimit`) (* (`self.TimeLimitIncrement`) _returnvalue)))
  (`KismetSystemLibrary.PrintString` (`KismetStringLibrary.Concat_StrStr` (`KismetStringLibrary.Conv_DoubleToString` _returnvalue_2) " - time of new round"))
  (return _returnvalue_2 (- (`self.BaseSpawnFrequency`) (* (`self.SpawnFrequencyDecrement`) _returnvalue))))

(fn `EndGame`
  (`Actor.K2_DestroyActor` (`self.CurrRound`)))

(fn `HandleRoundEnd`
  ; If we were Between Rounds  (ie waiting for the next combat round) we just move on to the next combat round. Otherwhise, tell GameMode that a round has ended.
  (if (`self.bBetweenRounds`)
    (`self.BeginNextRound`)
    (else
      (`self.RoundOver` (`self.CurrentRoundNumber`)))))

(fn `Init`
  (params (SelectedDifficulty :type "/Game/Data/F_DifficultySettings Structure") (SelectedTimeBetweenRounds :type "Float (double-precision)") (HUD :type "Array of /Game/UI/Widgets/Screens/WB_HUD Object Reference"))
  (bind (_roundstotal _basetimelimit _timitlimitincrement _basespawnfrequency _spawnfrequencydecrement) (break `/Game/Data/F_DifficultySettings` SelectedDifficulty))
  (bind _asbp_adv_game_instance (cast `/Game/BitWindy/Multiplayer/BP_AdvGameInstance` (`GameplayStatics.GetGameInstance`)))
  (`/Game/BitWindy/Multiplayer/BP_AdvGameInstance.ROS_CreateRound` _asbp_adv_game_instance)
  (set `self.CurrRound` (`/Game/BitWindy/Multiplayer/BP_AdvGameInstance.Current Round` _asbp_adv_game_instance))
  ; Internal Variable Set Up
  (set `self.TimeBetweenRounds` SelectedTimeBetweenRounds)
  (set `self.BaseTimeLimit` _basetimelimit)
  (set `self.BaseSpawnFrequency` _basespawnfrequency)
  (set `self.TimeLimitIncrement` _timitlimitincrement)
  (set `self.SpawnFrequencyDecrement` _spawnfrequencydecrement)
  ; HUD Event Binding
  (for _array_element (`local.HUD`)
    (add `self.RoundBegin` (`|CreateDelegate` _array_element :!event `OnRoundBegin`))
    (add `self.RoundOver` (`|CreateDelegate` _array_element :!event `OnRoundOver`)))
  ; GameState Event Binding
  (bind _asbp_tower_defense_game_state (cast `/Game/Blueprints/GameArchitecture/GameStates/BP_TowerDefense_GameState` (`GameplayStatics.GetGameState`))
    (:`then`
      (add `self.RoundBegin` (`|CreateDelegate` _asbp_tower_defense_game_state :!event `OnRoundBegin`))
      (add `self.RoundOver` (`|CreateDelegate` _asbp_tower_defense_game_state :!event `OnRoundEnd`)))
    (:`CastFailed`
      (`KismetSystemLibrary.RaiseScriptError` "Using Wrong Game State"))))

(fn `WaitForNextRound`
  (bind _timebetweenrounds (`self.TimeBetweenRounds`))
  (bind _currround (`self.CurrRound`))
  ; To avoid redundant logic, start a round with no enemies to act as the in between round timer
  (add `/Game/Blueprints/Actors/BP_Round.RoundTimerDone` _currround (`|CreateDelegate` :!event `OnRoundEnd`))
  (`/Game/Blueprints/Actors/BP_Round.Start` _currround _timebetweenrounds (+ _timebetweenrounds 1.0) true)
  (bind _output_get (set `self.bBetweenRounds` true))
  (`self.RoundBegin` (`self.CurrentRoundNumber`) (`self.TimeBetweenRounds`) _output_get))