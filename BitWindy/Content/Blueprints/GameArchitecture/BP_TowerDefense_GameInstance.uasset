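; Game instance for the tower defense game, holding game settings and the local player count alongside persistent menu audio.
; Init spawns 2D audio components for main and pause menus that survive level transitions, though the pause one has no sound assigned, then toggles on-screen messages by the Debugging flag.
; InitAudio re-runs that same chain.
; Simple setters and a getter expose the stored settings and player count.
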(event `self.ReceiveInit`
  (bind _returnvalue (`GameplayStatics.SpawnSound2D` "/Game/Audio/Metasounds/Sources/MS_SFX_UI_MainMenu.MS_SFX_UI_MainMenu" 1.0 1.0 0.0 null true :!label _label))
  (set `self.MS_UI_MainMenu` _returnvalue)
  (bind _returnvalue_2 (`GameplayStatics.SpawnSound2D` null 1.0 1.0 0.0 null true))
  (set `self.MS_UI_PauseMenu` _returnvalue_2)
  (if (`self.bDebugging?`)
    (`KismetSystemLibrary.ExecuteConsoleCommand` "EnableAllScreenMessages" null)
    (else
      (`KismetSystemLibrary.ExecuteConsoleCommand` "DisableAllScreenMessages" null))))

(event `InitAudio`
  (goto _label))

(event `/Game/Blueprints/GameArchitecture/BPI_TowerDefenseInst.SetSettings`
  (params (NewSettings :type "/Game/Blueprints/GameArchitecture/Settings/BP_GameSettings Class Reference"))
  (set `self.GameSettings` NewSettings))

(event `/Game/Blueprints/GameArchitecture/BPI_TowerDefenseInst.SetNumberOfLocalPlayers`
  (params (`Number Of Players` :type Integer))
  (set `self.NumberOfLocalPlayer` `Number Of Players`))

(fn `GetNumberOfLocalPlayers`
  (returns (`Number Of Local Players` :type Integer))
  (return (`self.NumberOfLocalPlayer`)))