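; Round manager component that alternates timed combat rounds with breaks, apparently for a King of the Hill mode.
; Breaks reuse the round object as a spawn-free countdown; when one ends, a new round is created through the game instance with time and spawn values scaled by round number.
; Init takes difficulty's base time and hard-codes scaling.
; Round begin/over events notify listeners; combat end waits for an AdvanceRounds call.
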(event `HandleRound`
  (bind _timebetweenrounds (`self.TimeBetweenRounds`))
  (bind _currround (`self.CurrRound`))
  (add `/Game/Blueprints/Actors/BP_Round.RoundTimerDone` _currround (`|CreateDelegate` :!event `OnRoundEnd`))
  (`/Game/Blueprints/Actors/BP_Round.Start` _currround _timebetweenrounds (+ _timebetweenrounds 1.0) true)
  (bind _output_get (set `self.bBetweenRounds` true))
  (`self.RoundBegin` (`self.CurrentRoundNumber`) (`self.TimeBetweenRounds`) _output_get))

(event `OnRoundEnd`
  (`self.HandleRoundEnd`))

(fn `AdvanceRounds`
  (`/Engine/EditorBlueprintResources/StandardMacros.IncrementInt` (`self.CurrentRoundNumber`)
    (:`  `
      (`self.WaitForNextRound`))))

(fn `BeginNextRound`
  (bind (_timelimit _spawnfrequency) (`self.CalculateNextRoundTimerParameters`))
  (bind _asbp_adv_game_instance (cast `/Game/BitWindy/Multiplayer/BP_AdvGameInstance` (`GameplayStatics.GetGameInstance`)))
  (`/Game/BitWindy/Multiplayer/BP_AdvGameInstance.ROS_CreateRound` _asbp_adv_game_instance)
  (bind _current_round (`/Game/BitWindy/Multiplayer/BP_AdvGameInstance.Current Round` _asbp_adv_game_instance))
  (add `/Game/Blueprints/Actors/BP_Round.RoundTimerDone` _current_round (`|CreateDelegate` :!event `OnRoundEnd`))
  (`/Game/Blueprints/Actors/BP_Round.Start` _current_round _timelimit _spawnfrequency false)
  (set `self.CurrRound` _current_round)
  (bind _output_get (set `self.bBetweenRounds` false))
  (`self.RoundBegin` (`self.CurrentRoundNumber`) _timelimit _output_get))

(fn `CalculateNextRoundTimerParameters`
  (returns (TimeLimit :type "Float (double-precision)") (SpawnFrequency :type "Float (double-precision)"))
  (bind _returnvalue (- (`self.CurrentRoundNumber`) 1))
  (bind _returnvalue_2 (+ (`self.BaseTimeLimit`) (* (`self.TimeLimitIncrement`) _returnvalue)))
  (`KismetSystemLibrary.PrintString` (`KismetStringLibrary.Concat_StrStr` (`KismetStringLibrary.Conv_DoubleToString` _returnvalue_2) " - time of new round"))
  (return _returnvalue_2 (- (`self.BaseSpawnFrequency`) (* (`self.SpawnFrequencyDecrement`) _returnvalue))))

(fn `EndGame`
  (`Actor.K2_DestroyActor` (`self.CurrRound`)))

(fn `HandleRoundEnd`
  (bind _currentroundnumber (`self.CurrentRoundNumber`))
  ; If we were Between Rounds  (ie waiting for the next combat round) we just move on to the next combat round. Otherwhise, tell GameMode that a round has ended.
  (if (`self.bBetweenRounds`)
    (`self.BeginNextRound`)
    (else
      (`KismetSystemLibrary.PrintString` (`KismetStringLibrary.Concat_StrStr` "Round number " (`KismetStringLibrary.Conv_IntToString` _currentroundnumber)))
      (`self.RoundOver` _currentroundnumber))))

(fn `Init`
  (params (SelectedDifficulty :type "/Game/Data/F_DifficultySettings Structure") (SelectedTimeBetweenRounds :type "Float (double-precision)") (HUD :type "/Game/UI/Widgets/Screens/WB_HUD_Domination Object Reference"))
  (bind _asbp_adv_game_instance (cast `/Game/BitWindy/Multiplayer/BP_AdvGameInstance` (`GameplayStatics.GetGameInstance`)))
  (`/Game/BitWindy/Multiplayer/BP_AdvGameInstance.ROS_CreateRound` _asbp_adv_game_instance)
  (bind _current_round (`/Game/BitWindy/Multiplayer/BP_AdvGameInstance.Current Round` _asbp_adv_game_instance))
  (set `self.CurrRound` _current_round)
  ; Internal Variable Set Up
  (set `self.TimeBetweenRounds` SelectedTimeBetweenRounds)
  (set `self.BaseTimeLimit` (`.BaseTimeLimit_6_C2F3704A41F257D706033D97D8DC7487` (break `/Game/Data/F_DifficultySettings` SelectedDifficulty)))
  (set `self.BaseSpawnFrequency` 100000.0)
  (set `self.TimeLimitIncrement` 0.0)
  (set `self.SpawnFrequencyDecrement` 100000.0)
  ; HUD Event Binding
  (add `/Game/Blueprints/Actors/BP_Round.RoundTimeTick` _current_round (`|CreateDelegate` (`local.HUD`) :!event `Set Timer Remaining in round`))
  (add `self.RoundBegin` (`|CreateDelegate` (`local.HUD`) :!event `OnRoundBegin`))
  (add `self.RoundOver` (`|CreateDelegate` (`local.HUD`) :!event `OnRoundOver`))
  ; GameState Event Binding
  (bind _asbp_gs_koth (cast `/Game/Blueprints/GameArchitecture/GameModes/KOTH/BP_GS_KOTH` (`GameplayStatics.GetGameState`)))
  (add `self.RoundBegin` (`|CreateDelegate` _asbp_gs_koth :!event `OnRoundBegin`)))

(fn `WaitForNextRound`
  (bind _timebetweenrounds (`self.TimeBetweenRounds`))
  (bind _currround (`self.CurrRound`))
  ; To avoid redundant logic, start a round with no enemies to act as the in between round timer
  (add `/Game/Blueprints/Actors/BP_Round.RoundTimerDone` _currround (`|CreateDelegate` :!event `OnRoundEnd`))
  (`/Game/Blueprints/Actors/BP_Round.Start` _currround _timebetweenrounds (+ _timebetweenrounds 1.0) true)
  (bind _output_get (set `self.bBetweenRounds` true))
  (`self.RoundBegin` (`self.CurrentRoundNumber`) (`self.TimeBetweenRounds`) _output_get))