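; Spawner bucket that holds a pool of spawners and picks one either at random or by least use.
; AddSpawner fills parallel Spawners and TimesChosen arrays and returns itself for chaining.
; GetRandomSpawner and GetLeastUsedSpawner increment a usage count and return a spawner.
; Both repeat their lookup after incrementing, so the returned spawner can differ from the one counted.
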(fn `AddSpawner`
  (params (Spawner :type "/Game/Blueprints/Actors/BP_EnemySpawner Object Reference"))
  (returns (BucketRef :type "/Game/Blueprints/GameArchitecture/Components/BP_SpawnerBucket Object Reference"))
  (`KismetArrayLibrary.Array_Add` (`self.Spawners`) Spawner)
  (`KismetArrayLibrary.Array_Add` (`self.TimesChosen`))
  (return self))

(fn `GetLeastUsedSpawner`
  (returns (Spawner :type "/Game/Blueprints/Actors/BP_EnemySpawner Object Reference"))
  (bind _indexofminvalue (`KismetMathLibrary.MinOfIntArray` (`self.TimesChosen`)))
  (`/Engine/EditorBlueprintResources/StandardMacros.IncrementInt` (`|GetArrayItem` (`self.TimesChosen`) _indexofminvalue)
    (:`  `
      (return (`|GetArrayItem` (`self.Spawners`) _indexofminvalue)))))

(fn `GetRandomSpawner`
  (returns (Spawner :type "/Game/Blueprints/Actors/BP_EnemySpawner Object Reference"))
  (bind (_outitem _outindex) (`KismetArrayLibrary.Array_Random` (`self.Spawners`)))
  (`/Engine/EditorBlueprintResources/StandardMacros.IncrementInt` (`|GetArrayItem` (`self.TimesChosen`) _outindex)
    (:`  `
      (return _outitem))))