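; Game mode for the tower defense shooter that runs the match from settings to win or loss.
; Construction reads difficulty and round timing from the game instance, then BeginPlay initializes the game state, binds tower destruction as the loss condition and starts the round manager.
; Completing the final round wins; both outcomes show screen text, end rounds and notify the music manager.
; Also provides player and bullet spawning helpers, while local multiplayer HUD setup is left unconnected.
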(event `self.K2_PostLogin`
  (params (NewPlayer :type "PlayerController Object Reference")))

(event `Initialize Rounds`
  (`self.SetUpRoundManager`)
  ; DO LAST - begin first round
  (`/Game/Blueprints/GameArchitecture/BP_RoundManager.AdvanceRounds` (`self.RoundManager`)))

(event `self.ReceiveBeginPlay`
  (`self.SetUpGameState`)
  (`self.Initialize Rounds`))

(event `Spawn Bullet`
  (params (Class :type "Actor Class Reference") (`Spawn Transform Location` :type "Vector Structure") (Owner :type "Actor Object Reference") (`Spawn Transform Rotation` :type "Rotator Structure") (Instigator :type "Pawn Object Reference"))
  (`|SpawnActorFromClass` Class (`KismetMathLibrary.MakeTransform` `Spawn Transform Location` `Spawn Transform Rotation`) "Undefined" "MultiplyWithRoot" Owner Instigator))

(fn `CheckForWin`
  (params (CurrentRound :type Integer))
  ;[0.1133 0.9062 0.1681 0.5] If we have not lost by the time the final round is completed, win the game
  (if (== CurrentRound (`.RoundsTotal_13_E8E21C214C75EC55D4F9F4876AE688B8` (break `/Game/Data/F_DifficultySettings` (`self.SelectedDifficultySettings`))))
    (`self.Win`)
    (else
      (`/Game/Blueprints/GameArchitecture/BP_RoundManager.AdvanceRounds` (`self.RoundManager`)))))

(fn `FindRandomPlayerStart`
  (returns (`Player Start Transform` :type "Transform Structure (by ref)"))
  (bind _outactors (`GameplayStatics.GetAllActorsOfClass` "/Script/Engine.PlayerStart"))
  (return (`self.GetTransform` (`|GetArrayItem` _outactors (`KismetMathLibrary.RandomIntegerInRange` 0 (- (`KismetArrayLibrary.Array_Length` _outactors) 1))))))

(fn `GetDifficultySettings`
  (returns (`Difficulty Settings` :type "/Game/Data/F_DifficultySettings Structure"))
  (return (`self.SelectedDifficultySettings`)))

(fn `GetIfRagdollingEnabled`
  (returns (bRagdollingEnabled :type Boolean))
  (return (`/Game/Blueprints/GameArchitecture/Settings/BP_GameSettings.bRagdolling` (`self.SelectedGameSettings`))))

(fn `GetWeaponOverride`
  (returns (Weapon :type "/Game/Variant_Shooter/Blueprints/Pickups/BP_ShooterWeaponBase Class Reference"))
  (return null))

(fn `Lose`
  (bind _number_of_local_players (message `/Game/Blueprints/GameArchitecture/BPI_TowerDefenseInst.GetNumberOfLocalPlayers` (`GameplayStatics.GetGameInstance`)))
  (for _index (range (+ _number_of_local_players 1))
    (bind _returnvalue (`|CreateWidget` "/Game/UI/Widgets/WB_CentreScreenText.WB_CentreScreenText_C" (`GameplayStatics.GetPlayerControllerFromID` _index) "You Lose!"))
    (`UserWidget.AddToPlayerScreen` _returnvalue 0))
  (`KismetSystemLibrary.PrintString` "Announcer Audio Here")
  (`self.Lost`)
  (bind _outactors (`GameplayStatics.GetAllActorsOfClass` "/Game/Variant_Shooter/Blueprints/AI/BP_ShooterNPC.BP_ShooterNPC_C"))
  (for _array_element _outactors
    (set `/Game/Variant_Shooter/Blueprints/AI/BP_ShooterNPC.bIsTargetEliminated` true _array_element))
  (`/Game/Blueprints/GameArchitecture/BP_RoundManager.EndGame` (`self.RoundManager`))
  (`/Game/Blueprints/GameArchitecture/BP_MusicManager.AnnounceLoss` (`self.BP_MusicManager`)))

(fn `Make HUD for player`
  (params (`player controller ID` :type Integer) (OwningPlayer :type "PlayerController Object Reference"))
  (bind _returnvalue (`|CreateWidget` "/Game/UI/Widgets/WB_HUD.WB_HUD_C" OwningPlayer))
  (`UserWidget.AddToPlayerScreen` _returnvalue 0)
  (bind _returnvalue_2 (`|CreateWidget` "/Game/Variant_Shooter/UI/UI_ShooterBulletCounter.UI_ShooterBulletCounter_C" OwningPlayer))
  (`UserWidget.AddToPlayerScreen` _returnvalue_2 0))

(fn `ParseSettings`
  (bind _asbp_adv_game_instance (cast `/Game/BitWindy/Multiplayer/BP_AdvGameInstance` (`GameplayStatics.GetGameInstance`)))
  (bind _gamesettings (`/Game/BitWindy/Multiplayer/BP_AdvGameInstance.GetGameSettings` _asbp_adv_game_instance))
  (bind _returnvalue (`|GenericCreateObject` _gamesettings))
  (bind _output_get (set `self.SelectedGameSettings` _returnvalue))
  (set `self.SelectedDifficultySettings` (`/Game/Blueprints/GameArchitecture/Settings/BP_GameSettings.DifficultySettings` _output_get))
  (set `self.SelectedTimeBetweenRounds` (`/Game/Blueprints/GameArchitecture/Settings/BP_GameSettings.TimeBetweenRounds` _output_get)))

(fn `SetUpGameState`
  ; This is now an unnecessary cast
  (bind _asbp_tower_defense_game_state (cast `/Game/Blueprints/GameArchitecture/BP_TowerDefense_GameState` (`GameplayStatics.GetGameState`))
    (:`then`
      (`/Game/Blueprints/GameArchitecture/BP_TowerDefense_GameState.InitDifficulty` _asbp_tower_defense_game_state (`self.SelectedDifficultySettings`) (`/Game/Blueprints/GameArchitecture/Settings/BP_GameSettings.PercentTowerHealthRecoveryBetweenRounds` (`self.SelectedGameSettings`)))
      ; Loss Condition Set Up
      (add `/Game/Blueprints/BP_Tower.TowerDestroyed` (`BlueprintMapLibrary.Map_Find` (`/Game/Blueprints/GameArchitecture/BP_TowerDefense_GameState.TowerMap` _asbp_tower_defense_game_state) "NewEnumerator0") (`|CreateDelegate` :!event `Lose`)))
    (:`CastFailed`
      (`KismetSystemLibrary.RaiseScriptError` "Not using TowerDefense GameState"))))

(fn `SetUpNewPlayerController`
  (bind _returnvalue (`GameplayStatics.CreatePlayer` -1))
  (bind _asbp_shooter_player_controller (cast `/Game/Variant_Shooter/Blueprints/BP_ShooterPlayerController` _returnvalue))
  (bind _returnvalue_2 (pcsubsystem `EnhancedInputLocalPlayerSubsystem` _asbp_shooter_player_controller))
  (`EnhancedInputSubsystemInterface.AddMappingContext` _returnvalue_2 "/Game/Input/IMC_Default.IMC_Default" 0 (struct))
  (`EnhancedInputSubsystemInterface.AddMappingContext` _returnvalue_2 "/Game/Variant_Shooter/Input/IMC_Weapons.IMC_Weapons" 0 (struct)))

(fn `SetUpRoundManager`
  (`/Game/Blueprints/GameArchitecture/BP_RoundManager.Init` (`self.RoundManager`) (`self.SelectedDifficultySettings`) (`self.SelectedTimeBetweenRounds`) (`self.Player_HUDs`))
  (add `/Game/Blueprints/GameArchitecture/BP_RoundManager.RoundOver` (`self.RoundManager`) (`|CreateDelegate` :!event `CheckForWin`)))

(fn `SpawnPlayer`
  (params (`Player Controller Reference` :type "/Game/Variant_Shooter/Blueprints/BP_ShooterPlayerController Object Reference"))
  (bind _returnvalue (`Controller.K2_GetPawn` `Player Controller Reference`))
  (`/Engine/EditorBlueprintResources/StandardMacros.IsValid` _returnvalue
    (:`Is Valid`
      (`self.K2_DestroyActor` _returnvalue))
    (:`Is Not Valid`
      _))
  (bind _returnvalue_2 (`|SpawnActorFromClass` "/Game/Variant_Shooter/Blueprints/BP_ShooterCharacter.BP_ShooterCharacter_C" (`self.FindRandomPlayerStart`) "Undefined" "MultiplyWithRoot" null null))
  (`Controller.Possess` `Player Controller Reference` _returnvalue_2))

(fn `UserConstructionScript`
  ; First
  (`self.ParseSettings`))

(fn `Win`
  (bind _number_of_local_players (message `/Game/Blueprints/GameArchitecture/BPI_TowerDefenseInst.GetNumberOfLocalPlayers` (`GameplayStatics.GetGameInstance`)))
  (for _index (range (+ _number_of_local_players 1))
    (bind _returnvalue (`|CreateWidget` "/Game/UI/Widgets/WB_CentreScreenText.WB_CentreScreenText_C" (`GameplayStatics.GetPlayerControllerFromID` _index) "You Won!"))
    (`UserWidget.AddToPlayerScreen` _returnvalue 0))
  (`KismetSystemLibrary.PrintString` "Announcer Audio Here")
  (`self.Won`)
  (`/Game/Blueprints/GameArchitecture/BP_RoundManager.EndGame` (`self.RoundManager`))
  (`/Game/Blueprints/GameArchitecture/BP_MusicManager.AnnounceWin` (`self.BP_MusicManager`))
  (bind _asbp_adv_game_instance (cast `/Game/BitWindy/Multiplayer/BP_AdvGameInstance` (`GameplayStatics.GetGameInstance`)))
  (`/Game/BitWindy/Multiplayer/BP_AdvGameInstance.End Game` _asbp_adv_game_instance))