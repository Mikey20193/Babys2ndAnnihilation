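; Tower defense GameState that tracks towers, remaining enemies, round number and local player count.
; Its construction script maps BP_Tower actors by name enum and binds to their health and the enemy spawner's count events, binding the spawner inside the tower loop.
; It relays tower health percentages and enemy counts through dispatchers.
; Round callbacks reset the enemy count at round end and restore a percentage of standing towers' health between rounds.
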(event `OnTowerHit`
  (params (CurrentTowerHealth :type "Float (double-precision)") (MaxTowerHealth :type "Float (double-precision)") (WhichTower :type "/Game/Data/ETower Enum" :default "NewEnumerator0"))
  ; Listeners
  (`self.PercentTowerHealthChanged` WhichTower (/ CurrentTowerHealth MaxTowerHealth)))

(event `IncreaseEnemyCount`
  ; Listeners
  (`/Engine/EditorBlueprintResources/StandardMacros.IncrementInt` (`self.EnemiesRemaining`)
    (:`  `
      (`self.EnemyCountChanged` (`self.EnemiesRemaining`) :!label _label))))

(event `DecreaseEnemyCount`
  ; Listeners
  (`/Engine/EditorBlueprintResources/StandardMacros.DecrementInt` (`self.EnemiesRemaining`)
    (:`  `
      (goto _label))))

(event `OnRoundBegin`
  (params (RoundNumber :type Integer) (TimeInRound :type "Float (double-precision)") (bBetweenRound :type Boolean))
  ; Listeners
  ;; Not currently used, may want to refactor round timing logic to go through state and not directly to HUD?
  (set `self.CurrentRoundNumber` RoundNumber)
  (bind _output_get (set `self.bWaitingForNextCombatRound` bBetweenRound))
  (if _output_get
    (`self.RecoverTowerHealthBetweenRounds`)))

(event `OnRoundEnd`
  (params (RoundNumber :type Integer))
  ; Listeners
  ;; Tell HUD to clear enemies remaining
  (bind _output_get (set `self.EnemiesRemaining` 0))
  (`self.EnemyCountChanged` _output_get))

(event `/Game/Blueprints/GameArchitecture/BPI_TowerDefenceGameState.SetNumberOfPlayer`
  (params (NumberOfPlayers :type Integer))
  (set `self.NumberOfLocalPlayers` NumberOfPlayers))

(fn `GetNumberOfPlayers`
  (returns (`Number of players` :type Integer))
  (return (`self.NumberOfLocalPlayers`)))

(fn `GetRoundNumber`
  (returns (RoundNumber :type Integer))
  (return (`self.CurrentRoundNumber`)))

(fn `GetTower`
  (params (`Tower Name` :type "/Game/Data/ETower Enum" :default "NewEnumerator0"))
  (returns (Tower :type "/Game/Blueprints/BP_Tower Object Reference"))
  (return (`BlueprintMapLibrary.Map_Find` (`self.TowerMap`) `Tower Name`)))

(fn `GetTowerLocation`
  (params (Tower :type "/Game/Data/ETower Enum" :default "NewEnumerator0"))
  (returns (Location :type "Vector Structure"))
  (return (`self.K2_GetActorLocation` (`BlueprintMapLibrary.Map_Find` (`self.TowerMap`) Tower))))

(fn `InitDifficulty`
  (params (DifficultySettings :type "/Game/Data/F_DifficultySettings Structure") (TowerHealthRecovery :type "Float (double-precision)" :default 1.0))
  (set `self.TotalNumberOfRounds` (`.RoundsTotal_13_E8E21C214C75EC55D4F9F4876AE688B8` (break `/Game/Data/F_DifficultySettings` DifficultySettings)))
  (set `self.CurrentRoundNumber` 1)
  (set `self.PercentTowerHealthRecovery` (`local.TowerHealthRecovery`)))

(fn `RecoverTowerHealthBetweenRounds`
  (bind _towermap (`self.TowerMap`))
  (bind _keys (`BlueprintMapLibrary.Map_Keys` _towermap))
  (for _array_element _keys
    (bind _value (`BlueprintMapLibrary.Map_Find` _towermap _array_element))
    ; Only recover still standing towers
    (if (not (`/Game/Blueprints/BP_Tower.bTowerDestroyed` _value))
      (bind _maxhealth (`/Game/Blueprints/BP_Tower.MaxHealth` _value))
      (bind _output_get (set `/Game/Blueprints/BP_Tower.CurrentHealth` (`KismetMathLibrary.FClamp` (+ (`/Game/Blueprints/BP_Tower.CurrentHealth` _value) (* (`self.PercentTowerHealthRecovery`) _maxhealth)) 0.0 _maxhealth) _value))
      ; Update In UI
      (`self.PercentTowerHealthChanged` _array_element (/ _output_get _maxhealth)))))

(fn `SetUpReferencesAndEvents`
  ; Create Map of Tower Objects accessible by their Enum Name
  (bind _outactors (`GameplayStatics.GetAllActorsOfClass` "/Game/Blueprints/BP_Tower.BP_Tower_C"))
  (for _array_element _outactors
    (`BlueprintMapLibrary.Map_Add` (`self.TowerMap`) (`/Game/Blueprints/BP_Tower.Tower Name` _array_element) _array_element)
    (add `/Game/Blueprints/BP_Tower.TowerHealthChanged` _array_element (`|CreateDelegate` :!event `OnTowerHit`))
    ; Enemy Spawn and KO event subscription
    (bind _returnvalue (`GameplayStatics.GetActorOfClass` "/Game/Blueprints/BP_EnemySpawnerManager.BP_EnemySpawnerManager_C"))
    (add `/Game/Blueprints/BP_EnemySpawnerManager.EnemyCountIncreased` _returnvalue (`|CreateDelegate` :!event `IncreaseEnemyCount`))
    (add `/Game/Blueprints/BP_EnemySpawnerManager.EnemyCountDecreased` _returnvalue (`|CreateDelegate` :!event `DecreaseEnemyCount`))))

(fn `UserConstructionScript`
  (`self.SetUpReferencesAndEvents`))