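; Tower defense game mode for a Chaos variant that powers up the player's shooter character.
; On BeginPlay it equips the rifle and scales walk and sprint speed by a movement multiplier.
; The jump velocity boost waits one tick to work around the character's own override.
; Getter functions expose the ragdoll setting, selected difficulty settings and the rifle as weapon override.
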(event `self.ReceiveBeginPlay`
  (`parent.ReceiveBeginPlay`)
  ; Change default weapon to full auto
  (bind _returnvalue (`GameplayStatics.GetActorOfClass` "/Game/Variant_Shooter/Blueprints/BP_ShooterCharacter.BP_ShooterCharacter_C"))
  (set `/Game/Variant_Shooter/Blueprints/BP_ShooterCharacter.Weapon Class` "/Game/Variant_Shooter/Blueprints/Pickups/Weapons/BP_ShooterWeapon_Rifle.BP_ShooterWeapon_Rifle_C" _returnvalue)
  (`/Game/Variant_Shooter/Blueprints/BP_ShooterCharacter.Update Equiped Weapon` _returnvalue)
  ; Increase Movement
  (set `/Game/Variant_Shooter/Blueprints/BP_ShooterCharacter.Walk Speed` (* (`/Game/Variant_Shooter/Blueprints/BP_ShooterCharacter.Walk Speed` _returnvalue) (`self.MovementMultiplier`)) _returnvalue)
  (set `/Game/Variant_Shooter/Blueprints/BP_ShooterCharacter.Sprint Speed` (* (`/Game/Variant_Shooter/Blueprints/BP_ShooterCharacter.Sprint Speed` _returnvalue) (`self.MovementMultiplier`)) _returnvalue)
  ;; workaround to override the shooter character override
  (`KismetSystemLibrary.DelayUntilNextTick`)
  (`/Game/Variant_Shooter/Blueprints/BP_ShooterCharacter.SetJumpVelocity` _returnvalue (* (`/Game/Variant_Shooter/Blueprints/BP_ShooterCharacter.Jump Velocity` _returnvalue) (`self.JumpMultiplier`))))

(fn `GetDifficultySettings`
  (returns (`Difficulty Settings` :type "/Game/Data/F_DifficultySettings Structure"))
  (return (`self.SelectedDifficultySettings`)))

(fn `GetIfRagdollingEnabled`
  (returns (bRagdollingEnabled :type Boolean))
  (return (`/Game/Blueprints/GameArchitecture/Settings/BP_GameSettings.bRagdolling` (`self.SelectedGameSettings`))))

(fn `GetWeaponOverride`
  (returns (Weapon :type "/Game/Variant_Shooter/Blueprints/Pickups/BP_ShooterWeaponBase Class Reference"))
  (return "/Game/Variant_Shooter/Blueprints/Pickups/Weapons/BP_ShooterWeapon_Rifle.BP_ShooterWeapon_Rifle_C"))

(fn `UserConstructionScript`
  (`parent.UserConstructionScript`))