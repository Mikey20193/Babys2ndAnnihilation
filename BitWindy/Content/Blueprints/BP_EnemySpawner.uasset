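; Tower defense enemy spawner that creates enemies around itself and aims them at an assigned target tower.
; On BeginPlay it caches tower locations from the GameState and listens for the target's destruction, after which new enemies target the centre tower instead.
; SpawnEnemy randomly offsets each spawn, passes attack and retreat locations by message, and attaches a particle effect.
; A sphere overlap fades charge audio for the player, gated by a flag set on successful spawn.
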(event `self.ReceiveBeginPlay`
  (`self.GetTowerInfo`))

(event `OnTargetTowerDestroyed`
  (set `self.bTargetTowerDestroyed` true))

(event `self.Sphere.OnComponentBeginOverlap`
  (params (OverlappedComponent :type "PrimitiveComponent Object Reference") (OtherActor :type "Actor Object Reference") (OtherComp :type "PrimitiveComponent Object Reference") (OtherBodyIndex :type Integer) (bFromSweep :type Boolean) (SweepResult :type "HitResult Structure (by ref)"))
  (if (== (`GameplayStatics.GetObjectClass` OtherActor) "/Game/Variant_Shooter/Blueprints/BP_ShooterCharacter.BP_ShooterCharacter_C")
    (if (`self.PlayerIsCharging?`)
      (`self.PlayChargeSound`)
      (else
        (`self.Stop Charge Sound`)))))

(event `self.Sphere.OnComponentEndOverlap`
  (params (OverlappedComponent :type "PrimitiveComponent Object Reference") (OtherActor :type "Actor Object Reference") (OtherComp :type "PrimitiveComponent Object Reference") (OtherBodyIndex :type Integer))
  (if (== (`GameplayStatics.GetObjectClass` OtherActor) "/Game/Variant_Shooter/Blueprints/BP_ShooterCharacter.BP_ShooterCharacter_C")
    (`self.Stop Charge Sound`)))

(fn `GetTowerInfo`
  (bind _asbp_tower_defense_game_state (cast `/Game/Blueprints/GameArchitecture/BP_TowerDefense_GameState` (`GameplayStatics.GetGameState`))
    (:`then`
      (bind _location (`/Game/Blueprints/GameArchitecture/BP_TowerDefense_GameState.GetTowerLocation` _asbp_tower_defense_game_state "NewEnumerator0"))
      (set `self.Centre Tower Location` _location)
      (bind _location_2 (`/Game/Blueprints/GameArchitecture/BP_TowerDefense_GameState.GetTowerLocation` _asbp_tower_defense_game_state (`self.TargetTower`)))
      (set `self.Target Tower Location` _location_2)
      (bind _tower (`/Game/Blueprints/GameArchitecture/BP_TowerDefense_GameState.GetTower` _asbp_tower_defense_game_state (`self.TargetTower`)))
      (add `/Game/Blueprints/BP_Tower.TowerDestroyed` _tower (`|CreateDelegate` :!event `OnTargetTowerDestroyed`)))
    (:`CastFailed`
      (`KismetSystemLibrary.RaiseScriptError` "UsingInvalidGameState"))))

(fn `PlayChargeSound`
  (`AudioComponent.FadeIn` (`self.Charge Audio`) 1.0 1.0 0.0 "Linear"))

(fn `Spawn Enemy `
  (returns (bSuccessful :type Boolean) (SpawnedEnemyRef :type "Actor Object Reference"))
  (bind _centre_tower_location (`self.Centre Tower Location`))
  (bind (_returnvalue_x _returnvalue_y) (`KismetMathLibrary.BreakVector` (`KismetMathLibrary.GreaterGreater_VectorRotator` (`KismetMathLibrary.MakeVector` (`self.Spawn Offset`)) (`KismetMathLibrary.RandomRotator` false))))
  (bind _returnvalue (`SceneComponent.K2_GetComponentLocation` (`self.DefaultSceneRoot`)))
  ; Instance the Enemy
  (bind _returnvalue_2 (`|SpawnActorFromClass` (`self.Enemy Class`) (`KismetMathLibrary.MakeTransform` (+ (`SceneComponent.K2_GetComponentLocation` (`self.DefaultSceneRoot`)) (`KismetMathLibrary.MakeVector` _returnvalue_x _returnvalue_y))) "Undefined" "MultiplyWithRoot" null null))
  (if (`KismetSystemLibrary.IsValid` _returnvalue_2)
    (if (`self.bTargetTowerDestroyed`)
      ; Enemy target move location set up
      (message `/Game/Variant_Shooter/Blueprints/AI/BPI_InitTowerDefenseEnemy.SetTargetLocations` _returnvalue_2 _centre_tower_location _centre_tower_location _returnvalue)
      (else
        (message `/Game/Variant_Shooter/Blueprints/AI/BPI_InitTowerDefenseEnemy.SetTargetLocations` _returnvalue_2 (`self.Target Tower Location`) (`self.Centre Tower Location`) _returnvalue)))
    ; Spawn in Particle Effect for ceremony/polish
    (`NiagaraFunctionLibrary.SpawnSystemAttached` (`self.SpawnParticleEffect`) (`Actor.RootComponent` _returnvalue_2) "None" (0.0 0.0 -80.0) (struct) "KeepRelativeOffset" true)
    (set `self.PlayerIsCharging?` true)
    (return true _returnvalue_2)
    (else
      (return false _returnvalue_2))))

(fn `Stop Charge Sound`
  (`AudioComponent.FadeOut` (`self.Charge Audio`) 3.0 0.0 "Linear"))

(fn `UserConstructionScript`)